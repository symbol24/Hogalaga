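; BP_MyBookKey is a physics-simulated key prop, apparently book-related, that tracks whether it has been picked up.
; BeginPlay enables physics on the static mesh.
; Tick polls whether the FlatComponent mode is HumanHand and sets HaspickedUp to match after a one-second Delay.
; OnIsActionComponent returns true for any component, so every part counts as an action component.
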(event EventBeginPlay
  (Physics|SetSimulatePhysics (Variables|Default|GetStaticMeshComponent) true))

(event Collision|EventActorBeginOverlap
  (params (OtherActor :type Actor%20Object%20Reference)))

(event EventTick
  (params (DeltaSeconds :type Float%20%28single-precision%29))
  (if (Utilities|Enum|Equal(Enum) (Variables|/Script/HelloNeighbor.FlatComponent|GetMode (Variables|Default|GetFlatComponent)) "FM_HumanHand")
    (Utilities|FlowControl|Delay 1.0)
    (Variables|Default|SetHaspickedUp true)
    (else
      (Utilities|FlowControl|Delay 1.0)
      (Variables|Default|SetHaspickedUp false))))

(fn ConstructionScript)

(fn OnIsActionComponent
  (params (Component :type Primitive%20Component%20Object%20Reference))
  (return true))