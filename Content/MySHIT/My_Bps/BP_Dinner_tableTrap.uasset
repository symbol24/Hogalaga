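; Dining table trap with a hinged latch that unlocks and swings when its linked BP_Switcher_2 is turned on.
; Tick polls the switch state, then sets IsOn and plays a one-time opening timeline with sound.
; Overlapping the Box enables E input, which line-traces from the human's camera.
; Hitting the table extension component plays a second rotation on the same scene component and destroys the trigger box.
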(event OnComponentBeginOverlap(Box)
  (params (OverlappedComponent :type Primitive%20Component%20Object%20Reference) (OtherActor :type Actor%20Object%20Reference) (OtherComp :type Primitive%20Component%20Object%20Reference) (OtherBodyIndex :type Integer) (bFromSweep :type Boolean) (SweepResult :type Hit%20Result%20Structure%20%28by%20ref%29))
  ;[1 1 1] Enabling E
  (Utilities|Casting|CastToBP_Human OtherActor)
  (if (not (Variables|Default|GetHasOpened))
    (Input|EnableInput (Game|GetPlayerController 0))))

(event OnComponentEndOverlap(Box)
  (params (OverlappedComponent :type Primitive%20Component%20Object%20Reference) (OtherActor :type Actor%20Object%20Reference) (OtherComp :type Primitive%20Component%20Object%20Reference) (OtherBodyIndex :type Integer))
  ;[1 1 1] Enabling E
  (Utilities|Casting|CastToBP_Human OtherActor)
  (Input|DisableInput (Game|GetPlayerController 0)))

(event Custom|UpDown
  (params (Component :type Primitive%20Component%20Object%20Reference))
  ;[1 1 1] Open Latch on Switcher
  ;[1 1 1] Open Latch On Raycast
  (if (== Component (Variables|Default|Gettable_with_extention_Box003))
    (if (not (Variables|Default|GetIsMoving))
      (Audio|PlaySound2D "/Game/Sounds/cutscenes/Act2/door_wood_creak_big_Cue.door_wood_creak_big_Cue" 2.0)
      (Variables|Default|SetIsMoving true)
      (bind _newtrack_0 (Timeline|Speed Play)
        (:Update
          (Transformation|SetRelativeRotation (Variables|Default|GetScene) (Math|Rotator|MakeRotator 0.0 _newtrack_0 0.0) false false)
          (Variables|Default|SetHasOpened true)
          (Components|DestroyComponent (Variables|Default|GetBox)))))))

(event Custom|OpenLatch
  ;[1 1 1] Open Latch on Switcher
  (Utilities|FlowControl|DoOnce false
    (:Completed
      (Audio|PlaySound2D "/Game/Sounds/cutscenes/Act2/big_wood_door_opening_Cue.big_wood_door_opening_Cue" 2.0)
      (bind _newtrack_2 (Timeline|New Play)
        (:Update
          (Transformation|SetRelativeRotation (Variables|Default|GetScene) (Math|Rotator|MakeRotator 0.0 _newtrack_2 0.0) false false))))))

(event EventTick
  (params (DeltaSeconds :type Float%20%28single-precision%29))
  ;[1 1 1] SwitcherCheck
  (Utilities|FlowControl|Sequence
    (:then_0
      (bind _asbp_human (Utilities|Casting|CastToBP_Human (Components|GetOwner (Variables|/Script/HelloNeighbor.Human|GetCamera (Variables|Default|GetBp_Human))))))
    (:then_1
      _))
  (bind _asbp_switcher_2 (Utilities|Casting|CastToBP_Switcher_2 (Components|GetOwner (Variables|/Game/Objects/BP_Objects/BP_Switcher_2.BP_Switcher_2_C|GetSwitch (Variables|Default|GetSwitcher_2)))))
  (if (Utilities|Enum|Equal(Enum) (Variables|/Script/HelloNeighbor.Tumbler|Getm_eState _asbp_switcher_2) "TUMBLER_ON")
    (Variables|Default|SetIsOn true)
    (CallFunction|OpenLatch)))

(event Input|KeyboardEvents|E
  (params (Key :type Key%20Structure))
  (bind _bp_human (Variables|Default|GetBp_Human))
  (bind _camera (Variables|/Script/HelloNeighbor.Human|GetCamera _bp_human))
  (bind _returnvalue (Transformation|GetWorldLocation _camera))
  ;[1 1 1] Raycast
  (:Pressed
    (if (Variables|Default|GetIsOn)
      (bind (_outhits _returnvalue_2) (Collision|MultiLineTraceByChannel _returnvalue (+ _returnvalue (* (Math|Vector|GetForwardVector _camera) 2e+02)) "TraceTypeQuery1" false (Utilities|Array|MakeArray (stale EventTick _asbp_human)) "None" false))
      (if _returnvalue_2
        (bind _asbp_dinner_table_trap (Utilities|Casting|CastToBP_Dinner_tableTrap (.HitActor (Collision|BreakHitResult (Utilities|Array|Get(acopy) _outhits)))))
        (CallFunction|UpDown _asbp_dinner_table_trap (.HitComponent (Collision|BreakHitResult (Utilities|Array|Get(acopy) _outhits))))))))

(fn ConstructionScript)