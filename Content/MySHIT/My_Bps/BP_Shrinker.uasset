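; BP_Shrinker is a trigger actor that shrinks the BP_Human character that overlaps it.
; On overlap it stores the character, then a DoOnce rescales the capsule to ChangeScale, so each instance fires only once.
; It then lowers the character's walk and run speeds and uses MoveComponentTo to shift the camera back along X and slightly up.
; The construction script and NewFunction_0 are empty.
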(event OnComponentBeginOverlap(Trigger)
  (params (OverlappedComponent :type Primitive%20Component%20Object%20Reference) (OtherActor :type Actor%20Object%20Reference) (OtherComp :type Primitive%20Component%20Object%20Reference) (OtherBodyIndex :type Integer) (bFromSweep :type Boolean) (SweepResult :type Hit%20Result%20Structure%20%28by%20ref%29))
  ;[1 1 1] ShrinkCharacter
  (bind _asbp_human (Utilities|Casting|CastToBP_Human OtherActor))
  (bind _output_get (Variables|Default|SetHuman _asbp_human))
  (Utilities|FlowControl|DoOnce false
    (:Completed
      (Transformation|SetWorldScale3D (Variables|/Script/Engine.Character|GetCapsuleComponent _output_get) (Variables|Default|GetChangeScale))
      (CallFunction|ChangeCharacterMovement)
      (Components|MoveComponentTo (Variables|/Script/HelloNeighbor.Human|GetCamera _output_get) (Math|Vector|MakeVector (+ (.x (Variables|/Script/Engine.SceneComponent|GetRelativeLocation (Variables|/Script/HelloNeighbor.Human|GetCamera _output_get))) -7e+01) (.y (Variables|/Script/Engine.SceneComponent|GetRelativeLocation (Variables|/Script/HelloNeighbor.Human|GetCamera _output_get))) (+ (.z (Variables|/Script/Engine.SceneComponent|GetRelativeLocation (Variables|/Script/HelloNeighbor.Human|GetCamera _output_get))) 15.0)) (Variables|/Script/Engine.SceneComponent|GetRelativeRotation (Variables|/Script/HelloNeighbor.Human|GetCamera _output_get)) false false 0.2 false))))

(event Custom|ChangeCharacterMovement
  (bind _human (Variables|Default|GetHuman))
  ;[1 1 1] SlowDownWhenShrunk
  (Variables|/Script/HelloNeighbor.Human|Setm_fWalkSpeed _human 2.5e+02)
  (Variables|/Script/HelloNeighbor.Human|Setm_fRunSpeed _human 5.5e+02)
  (Variables|/Script/Engine.CharacterMovementComponent|SetMaxWalkSpeed (Variables|/Script/Engine.Character|GetCharacterMovement _human) 2.5e+02))

(fn ConstructionScript)

(fn NewFunction0
  (params (NewParam :type Boolean)))