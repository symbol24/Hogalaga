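; BP_InstanceTester2_2 is a construction-script Blueprint that builds a row of randomly chosen static meshes, with its event graph unused.
; The XY length of EndPoint divided by MeshWidth sets the piece count.
; StartingMesh takes the first random mesh, and added components attach to it at MeshWidth steps along its local X.
; Picks come from ArrayMeshesToSpawn via a random stream, using separate StaticMeshComponents rather than instancing.
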(event EventBeginPlay)

(event Collision|EventActorBeginOverlap
  (params (OtherActor :type Actor%20Object%20Reference)))

(event EventTick
  (params (DeltaSeconds :type Float%20%28single-precision%29)))

(fn ConstructionScript
  (bind _endpoint (Variables|Default|GetEndPoint))
  (bind _meshwidth (Variables|Default|GetMeshWidth))
  (bind _returnvalue (* _endpoint "1.000000,1.000000, 0"))
  (bind _returnvalue_2 (Math|Vector|VectorLength _returnvalue))
  (bind _returnvalue_3 (/ _returnvalue_2 _meshwidth))
  (bind _returnvalue_4 (Math|Float|Round _returnvalue_3))
  (bind _returnvalue_5 (- _returnvalue_4 1))
  (Components|StaticMesh|SetStaticMesh (Variables|Default|GetStartingMesh) (Utilities|Array|Get(acopy) (Variables|Default|GetArrayMeshesToSpawn) (Math|Random|RandomIntegerinRangefromStream 0 (Variables|Default|GetAmount%20Of%20Meshes) (Variables|Default|GetStream))))
  (if (> _returnvalue_5 0) ; Do We Need To Spawn Any Meshes
    (for _index (range 1 _returnvalue_5)
      (bind _returnvalue_6 (AddComponent|AddStaticMeshComponent true))
      (Transformation|AttachComponentToComponent _returnvalue_6 (Variables|Default|GetStartingMesh) "None" "KeepWorld" "SnapToTarget" "KeepWorld" true)
      (Transformation|SetRelativeLocation _returnvalue_6 (Math|Vector|MakeVector (* _index (Variables|Default|GetMeshWidth)) 0.0 0.0) false false)
      (Components|StaticMesh|SetStaticMesh _returnvalue_6 (Utilities|Array|Get(acopy) (Variables|Default|GetArrayMeshesToSpawn) (Math|Random|RandomIntegerinRangefromStream 0 (Variables|Default|GetAmount%20Of%20Meshes) (Variables|Default|GetStream)))))))