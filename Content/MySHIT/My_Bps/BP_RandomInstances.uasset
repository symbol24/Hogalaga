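; BP_RandomInstances is an actor that scatters copies of a chosen static mesh across a flat square around its origin.
; The Construction Script loops NumberOfInstances times, adding a component at a seeded random X/Y offset and assigning TheMeshToUse to it and to TheMesh.
; Despite the name, each copy is a separate StaticMeshComponent, with no instanced mesh component used.
; The event graph holds no logic.
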(event EventBeginPlay)

(event Collision|EventActorBeginOverlap
  (params (OtherActor :type Actor%20Object%20Reference)))

(event EventTick
  (params (DeltaSeconds :type Float%20%28single-precision%29)))

(fn ConstructionScript
  (for _index (range 1 (Variables|Default|GetNumberOfInstances))
    (Components|StaticMesh|SetStaticMesh (Variables|Default|GetTheMesh) (Variables|Default|GetTheMeshToUse))
    (bind _returnvalue (AddComponent|AddStaticMeshComponent false (Math|Transform|MakeTransform (Math|Vector|MakeVector (Math|Random|RandomFloatinRangefromStream -5e+02 5e+02 (Variables|Default|GetStream)) (Math|Random|RandomFloatinRangefromStream -5e+02 5e+02 (Variables|Default|GetStream)) 0.0))))
    (Components|StaticMesh|SetStaticMesh _returnvalue (Variables|Default|GetTheMeshToUse))))