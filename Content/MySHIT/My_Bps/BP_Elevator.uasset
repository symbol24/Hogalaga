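; BP_Elevator is an elevator actor that starts moving when its linked BP_Switcher_2 is switched on.
; Each Tick it casts the owner of the Switcher's FlatComponent and checks for the TUMBLERON state, using DoOnce to fire MoveUp a single time.
; MoveUp plays a timeline that drives the root's relative location on the Y axis, despite the event's name, with no return movement.
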(event Custom|MoveUp
  (bind _newtrack_0 (Timeline|Timeline_0 Play)
    (:Update
      (Transformation|SetRelativeLocation (Variables|Default|GetDefaultSceneRoot) (Math|Vector|MakeVector 0.0 _newtrack_0 0.0) false false))))

(event EventBeginPlay)

(event Collision|EventActorBeginOverlap
  (params (OtherActor :type Actor%20Object%20Reference)))

(event EventTick
  (params (DeltaSeconds :type Float%20%28single-precision%29))
  (bind _asbp_switcher_2 (Utilities|Casting|CastToBP_Switcher_2 (Components|GetOwner (Variables|/Script/HelloNeighbor.FlatActor|GetFlatComponent (Variables|Default|GetSwitcher)))))
  (if (Utilities|Enum|Equal(Enum) (Variables|/Script/HelloNeighbor.Tumbler|Getm_eState _asbp_switcher_2) "TUMBLER_ON")
    (Utilities|FlowControl|DoOnce false
      (:Completed
        (CallFunction|MoveUp)))))

(fn ConstructionScript)