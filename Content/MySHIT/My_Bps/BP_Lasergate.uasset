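; Laser gate hazard that hurts a BP_Human player standing in its trigger box and drives a moving platform from electricity state.
; Load, begin play and connection changes open the platform when powered and close it otherwise, with OpenClose playing during movement.
; Overlap shows particles, plays a sizzle and sets a flag.
; Tick then drains HealthAsset's health through Delay nodes, resetting it and calling game mode Refresh at zero.
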(event OnChangeMovingState(Platform)
  (params (NewState :type EMovingState%20Enum :default "MS_OPEN"))
  (bind _open_close (Variables|Default|GetOpen/Close))
  (switch Utilities|FlowControl|Switch|SwitchonEMovingState NewState
    (:MS_OPEN
      (Audio|Components|Audio|Stop _open_close :!label _label))
    (:MS_CLOSE
      (goto _label))
    (:MS_OPENING
      (Audio|Components|Audio|Play _open_close 0.0 :!label _label_2))
    (:MS_CLOSING
      (goto _label_2))))

(event OnComponentBeginOverlap(Box)
  (params (OverlappedComponent :type Primitive%20Component%20Object%20Reference) (OtherActor :type Actor%20Object%20Reference) (OtherComp :type Primitive%20Component%20Object%20Reference) (OtherBodyIndex :type Integer) (bFromSweep :type Boolean) (SweepResult :type Hit%20Result%20Structure%20%28by%20ref%29))
  (Utilities|Casting|CastToBP_Human OtherActor)
  (Variables|Default|SetNewVar_0 true)
  (Rendering|SetVisibility (Variables|Default|GetParticleSystem) true false)
  (Audio|SpawnSound2D "/Game/Sounds/Objects/Noise/sizzle_burn_Cue.sizzle_burn_Cue"))

(event OnComponentEndOverlap(Box)
  (params (OverlappedComponent :type Primitive%20Component%20Object%20Reference) (OtherActor :type Actor%20Object%20Reference) (OtherComp :type Primitive%20Component%20Object%20Reference) (OtherBodyIndex :type Integer))
  (Utilities|Casting|CastToBP_Human OtherActor)
  (Variables|Default|SetNewVar_0 false)
  (Rendering|SetVisibility (Variables|Default|GetParticleSystem) false false))

(event EventOnChangeConnection
  (bind _platform (Variables|Default|GetPlatform))
  (bind _returnvalue (Class|MovingComponent|GetMovingState _platform))
  (if (Class|Electric|HasElectricity)
    (Utilities|FlowControl|Sequence
      (:then_0
        (Rendering|SetVisibility (Variables|Default|GetParticleSystem) false false)
        (switch Utilities|FlowControl|Switch|SwitchonEMovingState _returnvalue
          (:MS_CLOSE
            _)
          (:MS_CLOSING
            _))
        (Class|MovingComponent|SetMovingState (Variables|Default|GetPlatform) "MS_OPENING"))
      (:then_1
        (Utilities|Casting|CastToHealth (Components|GetOwner (Variables|/Hogalaga/MySHIT/My_Bps/Health.Health_C|GetDefaultSceneRoot (Variables|Default|GetHealthAsset))))
        (Utilities|FlowControl|Delay 0.5)
        (Variables|Default|SetNewhealth 1.0)))
    (else
      (switch Utilities|FlowControl|Switch|SwitchonEMovingState _returnvalue
        (:MS_OPEN
          _)
        (:MS_OPENING
          _))
      (Class|MovingComponent|SetMovingState (Variables|Default|GetPlatform) "MS_CLOSING"))))

(event EventBeginPlay
  (bind _platform (Variables|Default|GetPlatform))
  (bind _returnvalue (Class|MovingComponent|GetMovingState _platform))
  (if (Class|Electric|HasElectricity)
    (Utilities|FlowControl|Sequence
      (:then_0
        (Rendering|SetVisibility (Variables|Default|GetParticleSystem) false false)
        (switch Utilities|FlowControl|Switch|SwitchonEMovingState _returnvalue
          (:MS_CLOSE
            _)
          (:MS_CLOSING
            _))
        (Class|MovingComponent|SetMovingState (Variables|Default|GetPlatform) "MS_OPENING"))
      (:then_1
        (Utilities|Casting|CastToHealth (Components|GetOwner (Variables|/Hogalaga/MySHIT/My_Bps/Health.Health_C|GetDefaultSceneRoot (Variables|Default|GetHealthAsset))))
        (Utilities|FlowControl|Delay 0.5)
        (Variables|Default|SetNewhealth 1.0)))
    (else
      (switch Utilities|FlowControl|Switch|SwitchonEMovingState _returnvalue
        (:MS_OPEN
          _)
        (:MS_OPENING
          _))
      (Class|MovingComponent|SetMovingState (Variables|Default|GetPlatform) "MS_CLOSING"))))

(event EventTick
  (params (DeltaSeconds :type Float%20%28single-precision%29))
  (bind _ashealth (Utilities|Casting|CastToHealth (Components|GetOwner (Variables|/Hogalaga/MySHIT/My_Bps/Health.Health_C|GetDefaultSceneRoot (Variables|Default|GetHealthAsset)))))
  (if (Variables|Default|GetNewVar_0)
    (Development|PrintString (Utilities|String|ToString(Boolean) (Variables|Default|GetNewVar_0)))
    (Utilities|FlowControl|Delay 0.2)
    (Variables|/Hogalaga/MySHIT/My_Bps/Health.Health_C|SetHealth _ashealth (- (Variables|/Hogalaga/MySHIT/My_Bps/Health.Health_C|GetHealth _ashealth) 0.15))
    (Utilities|FlowControl|Sequence
      (:then_0
        (if (>= (Variables|/Hogalaga/MySHIT/My_Bps/Health.Health_C|GetHealth _ashealth) 0.2)
          (Utilities|FlowControl|Delay 0.35)
          (Audio|PlaySound2D "/Game/Sounds/Human/human_dead_2.human_dead_2")))
      (:then_1
        (if (<= (Variables|/Hogalaga/MySHIT/My_Bps/Health.Health_C|GetHealth _ashealth) 0.0)
          (Variables|Default|SetNewVar_0 false)
          (Audio|SpawnSound2D "/Game/Sounds/NeighborVoice/Voice-Male-Late_Thirties-Swear-Fuck-Angry.Voice-Male-Late_Thirties-Swear-Fuck-Angry")
          (Utilities|FlowControl|Delay 0.1)
          (bind _ashello_neighbor_reborn_game_mode (Utilities|Casting|CastToHelloNeighborRebornGameMode (Game|GetGameMode)))
          (Variables|/Hogalaga/MySHIT/My_Bps/Health.Health_C|SetHealth _ashealth 1.0)
          (Class|HelloNeighborRebornGameMode|Refresh _ashello_neighbor_reborn_game_mode))))))

(event EventOnPostLoad
  (bind _platform (Variables|Default|GetPlatform))
  (bind _returnvalue (Class|MovingComponent|GetMovingState _platform))
  (if (Class|Electric|HasElectricity)
    (Utilities|FlowControl|Sequence
      (:then_0
        (Rendering|SetVisibility (Variables|Default|GetParticleSystem) false false)
        (switch Utilities|FlowControl|Switch|SwitchonEMovingState _returnvalue
          (:MS_CLOSE
            _)
          (:MS_CLOSING
            _))
        (Class|MovingComponent|SetMovingState (Variables|Default|GetPlatform) "MS_OPENING"))
      (:then_1
        (Utilities|Casting|CastToHealth (Components|GetOwner (Variables|/Hogalaga/MySHIT/My_Bps/Health.Health_C|GetDefaultSceneRoot (Variables|Default|GetHealthAsset))))
        (Utilities|FlowControl|Delay 0.5)
        (Variables|Default|SetNewhealth 1.0)))
    (else
      (switch Utilities|FlowControl|Switch|SwitchonEMovingState _returnvalue
        (:MS_OPEN
          _)
        (:MS_OPENING
          _))
      (Class|MovingComponent|SetMovingState (Variables|Default|GetPlatform) "MS_CLOSING"))))

(fn ConstructionScript)