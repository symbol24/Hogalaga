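; Level-streaming actor that rotates the world through three cycle sublevels each time the game saves.
; On BeginPlay it binds to the Hello Neighbor Reborn game mode's post-save event and streams in ThirdCycle.
; Each save advances a DoN counter, unloading the current sublevel and loading the next: First, Second, then Third.
; Loading ThirdCycle again resets the counter, so the rotation repeats.
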(event Custom|LoadLevels
  (bind _secondcycle (Variables|Default|GetSecondCycle))
  (bind _firstcycle (Variables|Default|GetFirstCycle))
  (bind _thirdcycle (Variables|Default|GetThirdCycle))
  (bind _returnvalue (Utilities|Name|MakeLiteralName _firstcycle))
  (bind _returnvalue_2 (Utilities|Name|MakeLiteralName _secondcycle))
  (bind _returnvalue_3 (Utilities|Name|MakeLiteralName _thirdcycle))
  (bind _counter (Utilities|FlowControl|DoN 3 :!label _label)
    (:Exit
      (switch int _counter
        (:1
          (Game|UnloadStreamLevel(byName) _returnvalue_3)
          (Game|LoadStreamLevel(byName) _returnvalue true))
        (:2
          (Game|UnloadStreamLevel(byName) _returnvalue)
          (Game|LoadStreamLevel(byName) _returnvalue_2 true))
        (:3
          (Game|UnloadStreamLevel(byName) _returnvalue_2)
          (Game|LoadStreamLevel(byName) _returnvalue_3 true)
          (goto _label Reset))))))

(event EventBeginPlay
  (bind _secondcycle (Variables|Default|GetSecondCycle))
  (bind _firstcycle (Variables|Default|GetFirstCycle))
  (bind _thirdcycle (Variables|Default|GetThirdCycle))
  (bind _returnvalue (Utilities|Name|MakeLiteralName _firstcycle))
  (bind _returnvalue_2 (Utilities|Name|MakeLiteralName _secondcycle))
  (bind _returnvalue_3 (Utilities|Name|MakeLiteralName _thirdcycle))
  (bind _ashello_neighbor_reborn_game_mode (Utilities|Casting|CastToHelloNeighborRebornGameMode (Game|GetGameMode)))
  (EventDispatchers|BindEventtoOnPostSave _ashello_neighbor_reborn_game_mode (delegate Custom|LoadLevels))
  (Game|LoadStreamLevel(byName) _returnvalue_3 true)
  (Utilities|FlowControl|DoN 3) ; enters at Reset
)

(fn ConstructionScript)