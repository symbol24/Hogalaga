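; BP_Potions is a pickup that restores health when held in the human player's hand.
; Tick polls the FlatComponent mode, then after delays plays a bite sound, hides the mesh and sets the first Health actor's value to 1.0.
; It then drives BP_Human through a throw hand state and animation before emptying the hand.
; The DestroyActor call is unwired, so the potion is only hidden.
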(event EventTick
  (params (DeltaSeconds :type Float%20%28single-precision%29))
  (if (Utilities|Enum|Equal(Enum) (Variables|/Script/HelloNeighbor.FlatComponent|GetMode (Variables|Default|GetFlatComponent)) "FM_HumanHand")
    (Variables|Default|SetWasPickedUp true)
    (Utilities|FlowControl|Delay 1.0)
    (Audio|PlaySound2D "/Hogalaga/MySHIT/Sounds/Biting_Apple-SoundBible_com-415478302.Biting_Apple-SoundBible_com-415478302")
    (Rendering|SetVisibility (Variables|Default|GetStaticMeshComponent) false false)
    (bind _outactors (Actor|GetAllActorsOfClass "/Hogalaga/MySHIT/My_Bps/Health.Health_C"))
    (Variables|/Hogalaga/MySHIT/My_Bps/Health.Health_C|SetHealth (Utilities|Array|Get(acopy) _outactors) 1.0)
    (Utilities|FlowControl|Delay 0.5)
    (bind _asbp_human (Utilities|Casting|CastToBP_Human (Game|GetPlayerCharacter 0)))
    (Class|Human|SetHandsState _asbp_human "HS_THROW")
    (Components|Animation|SetAnimation (Variables|/Script/Engine.Character|GetMesh _asbp_human) "/Game/Player/hands/player_body_Anim_rig_throw_banana.player_body_Anim_rig_throw_banana")
    (Utilities|FlowControl|Delay 0.5)
    (Class|Human|SetHandsState _asbp_human "HS_EMPTY")
    (Components|Animation|SetAnimation (Variables|/Script/Engine.Character|GetMesh _asbp_human) 0)))

(fn ConstructionScript)

(fn OnIsActionComponent
  (params (Component :type Primitive%20Component%20Object%20Reference))
  (return true))