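; BP_MyNewbUTTON is a toggle switch actor that keeps an on/off tumbler state in step with an animated Switch component.
; Action events and hits on Switch reverse its opening or closing motion, with a sound cue when actioned from a settled position.
; Tumbler changes drive the Switch, and its settled states write back to the tumbler, with equality checks guarding both directions.
; Construction and BeginPlay align the Switch to the tumbler state.
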(event OnChangeMovingState(Switch)
  (params (NewState :type EMovingState%20Enum :default "MS_OPEN"))
  (bind _returnvalue (Class|Tumbler|GetTumblerState))
  (switch Utilities|FlowControl|Switch|SwitchonEMovingState NewState
    (:MS_OPEN
      (if (Utilities|Enum|NotEqual(Enum) _returnvalue "TUMBLER_ON")
        (Class|Tumbler|SetTumblerState "TUMBLER_ON")))
    (:MS_CLOSE
      (if (Utilities|Enum|NotEqual(Enum) _returnvalue "TUMBLER_OFF")
        (Class|Tumbler|SetTumblerState "TUMBLER_OFF")))))

(event EventBeginPlay
  (bind _switch (Variables|Default|GetSwitch))
  ;[1 1 1] Comment
  (switch Utilities|FlowControl|Switch|SwitchonETumblerState (Class|Tumbler|GetTumblerState)
    (:TUMBLER_ON
      (Class|MovingComponent|SetMovingState _switch "MS_OPENING"))
    (:TUMBLER_OFF
      (Class|MovingComponent|SetMovingState _switch "MS_CLOSING"))))

(event Collision|EventHit
  (params (MyComp :type Primitive%20Component%20Object%20Reference) (Other :type Actor%20Object%20Reference) (OtherComp :type Primitive%20Component%20Object%20Reference) (bSelfMoved :type Boolean) (HitLocation :type Vector :default "0, 0, 0") (HitNormal :type Vector :default "0, 0, 0") (NormalImpulse :type Vector :default "0, 0, 0") (Hit :type Hit%20Result%20Structure%20%28by%20ref%29))
  (bind _switch (Variables|Default|GetSwitch))
  (if (== MyComp (Variables|Default|GetSwitch))
    (switch Utilities|FlowControl|Switch|SwitchonEMovingState (Class|MovingComponent|GetMovingState (Variables|Default|GetSwitch))
      (:MS_OPEN
        (Class|MovingComponent|SetMovingState _switch "MS_CLOSING" :!label _label))
      (:MS_CLOSE
        (Class|MovingComponent|SetMovingState _switch "MS_OPENING" :!label _label_2))
      (:MS_OPENING
        (goto _label))
      (:MS_CLOSING
        (goto _label_2)))))

(event EventOnChangeTumblerState
  (params (NewState :type ETumblerState%20Enum :default "TUMBLER_ON"))
  (bind _switch (Variables|Default|GetSwitch))
  (bind _switch_2 (Variables|Default|GetSwitch))
  (bind _returnvalue (Class|MovingComponent|GetMovingState _switch))
  ;[1 1 1] Comment
  (switch Utilities|FlowControl|Switch|SwitchonETumblerState NewState
    (:TUMBLER_ON
      (if (Utilities|Enum|NotEqual(Enum) _returnvalue "MS_OPEN")
        (Class|MovingComponent|SetMovingState _switch_2 "MS_OPENING")))
    (:TUMBLER_OFF
      (if (Utilities|Enum|NotEqual(Enum) _returnvalue "MS_CLOSE")
        (Class|MovingComponent|SetMovingState _switch_2 "MS_CLOSING")))))

(event EventOnEventAction
  (params (ActionMaker :type Actor%20Object%20Reference) (SpecialComponent :type Primitive%20Component%20Object%20Reference))
  (bind _switch (Variables|Default|GetSwitch))
  ;[1 1 1] Comment
  (if (== SpecialComponent (Variables|Default|GetSwitch))
    (switch Utilities|FlowControl|Switch|SwitchonEMovingState (Class|MovingComponent|GetMovingState (Variables|Default|GetSwitch))
      (:MS_OPEN
        (Class|MovingComponent|SetMovingState _switch "MS_CLOSING")
        (Audio|Components|Audio|Play (Variables|Default|Gettrain_room_button_Cue) 0.0 :!label _label))
      (:MS_CLOSE
        (Class|MovingComponent|SetMovingState _switch "MS_OPENING")
        (goto _label))
      (:MS_OPENING
        (Class|MovingComponent|SetMovingState _switch "MS_CLOSING"))
      (:MS_CLOSING
        (Class|MovingComponent|SetMovingState _switch "MS_OPENING")))))

(fn ConstructionScript
  (bind _switch (Variables|Default|GetSwitch))
  (switch Utilities|FlowControl|Switch|SwitchonETumblerState (Class|Tumbler|GetTumblerState)
    (:TUMBLER_ON
      (Class|MovingComponent|SetMovingState _switch "MS_OPENING"))
    (:TUMBLER_OFF
      (Class|MovingComponent|SetMovingState _switch "MS_CLOSING"))))

(fn OnIsActionComponent
  (params (Component :type Primitive%20Component%20Object%20Reference))
  (return true))