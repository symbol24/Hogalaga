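; Elevator actor that carries the player between a lobby and up to three upper floors.
; Inside its trigger, pressing E line-traces from the player camera and passes the hit component to UpDown.
; Door hits toggle three sliding panels; with doors open, button hits close them, move the root via MoveComponentTo, then reopen on arrival.
; CurrentHeight and WhatFloorImOn track position, while the construction script reveals upper-floor buttons from MaxStories.
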(event OnComponentBeginOverlap(Trigger)
  (params (OverlappedComponent :type Primitive%20Component%20Object%20Reference) (OtherActor :type Actor%20Object%20Reference) (OtherComp :type Primitive%20Component%20Object%20Reference) (OtherBodyIndex :type Integer) (bFromSweep :type Boolean) (SweepResult :type Hit%20Result%20Structure%20%28by%20ref%29))
  ;[1 1 1] Overlay Inout
  (Utilities|Casting|CastToBP_Human OtherActor)
  (Input|EnableInput (Game|GetPlayerController 0)))

(event OnComponentEndOverlap(Trigger)
  (params (OverlappedComponent :type Primitive%20Component%20Object%20Reference) (OtherActor :type Actor%20Object%20Reference) (OtherComp :type Primitive%20Component%20Object%20Reference) (OtherBodyIndex :type Integer))
  ;[1 1 1] Overlay Inout
  (Utilities|Casting|CastToBP_Human OtherActor)
  (Input|DisableInput (Game|GetPlayerController 0)))

(event Custom|Testcustom
  (params (Component :type Primitive%20Component%20Object%20Reference)))

(event Custom|OpenDoors
  (params (Component :type Primitive%20Component%20Object%20Reference))
  (bind _lift_door (Variables|Default|Getlift_door))
  (bind _lift_door1 (Variables|Default|Getlift_door1))
  (bind _staticmesh (Variables|Default|GetStaticMesh))
  (bind _lift_door1_2 (Variables|Default|Getlift_door1))
  (bind _lift_door_2 (Variables|Default|Getlift_door))
  (bind _staticmesh_2 (Variables|Default|GetStaticMesh))
  (bind _returnvalue (Transformation|GetRelativeTransform _lift_door_2))
  (bind _returnvalue_2 (Transformation|GetRelativeTransform _staticmesh))
  (bind _returnvalue_3 (Transformation|GetRelativeTransform _lift_door1_2))
  (bind _returnvalue_4 (Transformation|GetRelativeTransform _staticmesh_2))
  (bind _returnvalue_5 (Transformation|GetRelativeTransform _lift_door))
  (bind _returnvalue_6 (Transformation|GetRelativeTransform _lift_door1))
  ;[0.2218 1 0] AutoClose/Open
  (if (Variables|Default|GetJustOpened)
    (Utilities|FlowControl|Sequence
      (:then_0
        ;[0 0.3627 1] CloseDoors
        (Components|MoveComponentTo _lift_door1_2 (Math|Vector|MakeVector (+ (.x (.location _returnvalue_3)) 1.5e+02) (.y (.location _returnvalue_3)) (.z (.location _returnvalue_3))) (.rotation _returnvalue_3) true true 1.0 false))
      (:then_1
        (Components|MoveComponentTo _staticmesh (Math|Vector|MakeVector (+ (.x (.location _returnvalue_2)) 5e+01) (.y (.location _returnvalue_2)) (.z (.location _returnvalue_2))) (.rotation _returnvalue_2) true true 1.0 false))
      (:then_2
        (Components|MoveComponentTo _lift_door_2 (Math|Vector|MakeVector (+ (.x (.location _returnvalue)) 1e+02) (.y (.location _returnvalue)) (.z (.location _returnvalue))) (.rotation _returnvalue) true true 1.0 false)))
    (Variables|Default|SetIsMoving false)
    (Variables|Default|SetJustOpened false)
    ;[0 0.3627 1] OpenDoors
    (Utilities|FlowControl|DoOnce false) ; enters at Reset
    (else
      (Utilities|FlowControl|Sequence
        (:then_0
          (Components|MoveComponentTo _staticmesh_2 (Math|Vector|MakeVector (- (.x (.location _returnvalue_4)) 5e+01) (.y (.location _returnvalue_4)) (.z (.location _returnvalue_4))) (.rotation _returnvalue_4) true true 1.0 false))
        (:then_1
          (Components|MoveComponentTo _lift_door1 (Math|Vector|MakeVector (- (.x (.location _returnvalue_6)) 1.5e+02) (.y (.location _returnvalue_6)) (.z (.location _returnvalue_6))) (.rotation _returnvalue_6) true true 1.0 false))
        (:then_2
          (Components|MoveComponentTo _lift_door (Math|Vector|MakeVector (- (.x (.location _returnvalue_5)) 1e+02) (.y (.location _returnvalue_5)) (.z (.location _returnvalue_5))) (.rotation _returnvalue_5) true true 1.0 false)))
      (Variables|Default|SetIsMoving false)
      (Variables|Default|SetJustOpened true)
      (Utilities|FlowControl|DoOnce false) ; enters at Reset
    )))

(event Custom|UpDown
  (params (Component :type Primitive%20Component%20Object%20Reference))
  (bind _defaultsceneroot (Variables|Default|GetDefaultSceneRoot))
  (bind _lift_door (Variables|Default|Getlift_door))
  (bind _lift_door1 (Variables|Default|Getlift_door1))
  (bind _staticmesh (Variables|Default|GetStaticMesh))
  (bind _lift_door1_2 (Variables|Default|Getlift_door1))
  (bind _lift_door_2 (Variables|Default|Getlift_door))
  (bind _defaultsceneroot_2 (Variables|Default|GetDefaultSceneRoot))
  (bind _elevatorspeed (Variables|Default|GetElevatorSpeed))
  (bind _defaultsceneroot_3 (Variables|Default|GetDefaultSceneRoot))
  (bind _staticmesh_2 (Variables|Default|GetStaticMesh))
  (bind _defaultsceneroot_4 (Variables|Default|GetDefaultSceneRoot))
  (bind _returnvalue (Transformation|GetWorldLocation _defaultsceneroot_4))
  (bind _returnvalue_2 (Transformation|GetWorldRotation _defaultsceneroot_4))
  (bind _returnvalue_3 (Transformation|GetRelativeTransform _lift_door_2))
  (bind _returnvalue_4 (Transformation|GetRelativeTransform _staticmesh))
  (bind _returnvalue_5 (Transformation|GetRelativeTransform _lift_door1_2))
  (bind _returnvalue_6 (Transformation|GetWorldLocation _defaultsceneroot_2))
  (bind _returnvalue_7 (Transformation|GetWorldLocation _defaultsceneroot))
  (bind _returnvalue_8 (Transformation|GetWorldLocation _defaultsceneroot_3))
  (bind _returnvalue_9 (Transformation|GetWorldLocation _defaultsceneroot_3))
  (bind _returnvalue_10 (Transformation|GetWorldLocation _defaultsceneroot_2))
  (bind _returnvalue_11 (Transformation|GetRelativeTransform _staticmesh_2))
  (bind _returnvalue_12 (Transformation|GetRelativeTransform _lift_door))
  (bind _returnvalue_13 (Transformation|GetRelativeTransform _lift_door1))
  (Development|PrintString (Utilities|GetDisplayName Component))
  (Utilities|FlowControl|Sequence
    (:then_0
      (if (Variables|Default|GetJustOpened)
        (Utilities|FlowControl|Sequence
          (:then_0
            ;[1 0.1113 0.2816] FirstFloor
            (if (not (Variables|Default|GetIsMoving))
              (if (== Component (Variables|Default|GetUpButton))
                (if (Variables|Default|GetJustOpened)
                  (CallFunction|OpenDoors)
                  (Utilities|FlowControl|Delay 2.0))
                (Utilities|FlowControl|Sequence
                  (:then_0
                    (if (< (Variables|Default|GetCurrentHeight) (Variables|Default|GetTheStoryHeight))
                      (Variables|Default|SetIsMoving true)
                      (Components|MoveComponentTo _defaultsceneroot_2 (Math|Vector|MakeVector (.x _returnvalue_6) (.y _returnvalue_6) (+ (.z _returnvalue_6) (Variables|Default|GetTheStoryHeight))) (Transformation|GetWorldRotation _defaultsceneroot_2) true true (Variables|Default|GetElevatorSpeed) false)
                      (Variables|Default|SetCurrentHeight (+ (Variables|Default|GetCurrentHeight) (Variables|Default|GetTheStoryHeight)))
                      (Variables|Default|SetIsMoving false)
                      (Variables|Default|SetWhatFloorImOn 1)
                      (Utilities|FlowControl|Delay 1.0)
                      (CallFunction|OpenDoors)))
                  (:then_1
                    (if (not (<= (Variables|Default|GetWhatFloorImOn) 1))
                      (Variables|Default|SetIsMoving true)
                      (Components|MoveComponentTo _defaultsceneroot_2 (Math|Vector|MakeVector (.x _returnvalue_10) (.y _returnvalue_10) (- (.z _returnvalue_10) (- (* (Variables|Default|GetWhatFloorImOn) (Variables|Default|GetTheStoryHeight)) (Variables|Default|GetTheStoryHeight)))) (Transformation|GetWorldRotation _defaultsceneroot_2) true true (Variables|Default|GetElevatorSpeed) false)
                      (Variables|Default|SetCurrentHeight (- (Variables|Default|GetCurrentHeight) (- (* (Variables|Default|GetWhatFloorImOn) (Variables|Default|GetTheStoryHeight)) (Variables|Default|GetTheStoryHeight))))
                      (Variables|Default|SetIsMoving false)
                      (Variables|Default|SetWhatFloorImOn 1)
                      (Utilities|FlowControl|Delay 1.0)
                      (CallFunction|OpenDoors)))))))
          (:then_1
            ;[1 0.1113 0.2816] SecondFloor
            (if (not (Variables|Default|GetIsMoving))
              (if (> (Variables|Default|GetStoryHeight) 501.0)
                (if (== Component (Variables|Default|GetUpButton2))
                  (if (Variables|Default|GetJustOpened)
                    (CallFunction|OpenDoors)
                    (Utilities|FlowControl|Delay 2.0))
                  (if (<= (Variables|Default|GetCurrentHeight) (Variables|Default|GetStoryHeight))
                    (if (== (Variables|Default|GetWhatFloorImOn) 3)
                      (Variables|Default|SetIsMoving true)
                      (Components|MoveComponentTo _defaultsceneroot_3 (Math|Vector|MakeVector (.x _returnvalue_9) (.y _returnvalue_9) (- (.z _returnvalue_9) (- (* (Variables|Default|GetWhatFloorImOn) (Variables|Default|GetTheStoryHeight)) (* (Variables|Default|GetTheStoryHeight) 2.0)))) (Transformation|GetWorldRotation _defaultsceneroot_3) true true (Variables|Default|GetElevatorSpeed) false)
                      (Variables|Default|SetCurrentHeight (- (Variables|Default|GetCurrentHeight) (- (* (Variables|Default|GetWhatFloorImOn) (Variables|Default|GetTheStoryHeight)) (* (Variables|Default|GetTheStoryHeight) 2.0))))
                      (Variables|Default|SetIsMoving false)
                      (Variables|Default|SetWhatFloorImOn 2)
                      (CallFunction|OpenDoors)
                      (else
                        (Variables|Default|SetIsMoving true)
                        (Components|MoveComponentTo _defaultsceneroot_3 (Math|Vector|MakeVector (.x _returnvalue_8) (.y _returnvalue_8) (- (.z _returnvalue_8) (- (* (Variables|Default|GetWhatFloorImOn) (Variables|Default|GetTheStoryHeight)) (* (Variables|Default|GetTheStoryHeight) 2.0)))) (Transformation|GetWorldRotation _defaultsceneroot_3) true true (* (Variables|Default|GetElevatorSpeed) 2.0) false)
                        (Variables|Default|SetCurrentHeight (+ (Variables|Default|GetCurrentHeight) (- (* (Variables|Default|GetTheStoryHeight) 2.0) (Variables|Default|GetCurrentHeight))))
                        (Variables|Default|SetIsMoving false)
                        (Variables|Default|SetWhatFloorImOn 2)
                        (CallFunction|OpenDoors))))))))
          (:then_2
            ;[1 0.2596 0.01202] Lobby
            (if (== Component (Variables|Default|GetDownButton))
              (if (Variables|Default|GetJustOpened)
                (CallFunction|OpenDoors)
                (Utilities|FlowControl|Delay 2.0))
              (if (> (Variables|Default|GetCurrentHeight) (Variables|Default|GetMinimumHeight))
                (Variables|Default|SetIsMoving true)
                (if (< (Variables|Default|GetCurrentHeight) 501.0)
                  (Components|MoveComponentTo _defaultsceneroot_4 (Math|Vector|MakeVector (.x _returnvalue) (.y _returnvalue) (- (.z _returnvalue) (Variables|Default|GetCurrentHeight))) _returnvalue_2 true true _elevatorspeed false)
                  (else
                    (Components|MoveComponentTo _defaultsceneroot_4 (Math|Vector|MakeVector (.x _returnvalue) (.y _returnvalue) (- (.z _returnvalue) (Variables|Default|GetCurrentHeight))) _returnvalue_2 true true (* _elevatorspeed (Variables|Default|GetMaxStories)) false)))
                (Variables|Default|SetCurrentHeight (- (Variables|Default|GetCurrentHeight) (Variables|Default|GetCurrentHeight)))
                (Variables|Default|SetIsMoving false)
                (Variables|Default|SetWhatFloorImOn 0)
                (CallFunction|OpenDoors))))
          (:then_3
            ;[1 0.1113 0.2816] 3rdFloor
            (if (not (Variables|Default|GetIsMoving))
              (if (== Component (Variables|Default|GetUpbuttoon3))
                (if (Variables|Default|GetJustOpened)
                  (CallFunction|OpenDoors)
                  (Utilities|FlowControl|Delay 2.0))
                (if (< (Variables|Default|GetCurrentHeight) (Variables|Default|GetStoryHeight))
                  (Variables|Default|SetIsMoving true)
                  (Components|MoveComponentTo _defaultsceneroot (Math|Vector|MakeVector (.x _returnvalue_7) (.y _returnvalue_7) (+ (.z _returnvalue_7) (- (Variables|Default|GetStoryHeight) (Variables|Default|GetCurrentHeight)))) (Transformation|GetWorldRotation _defaultsceneroot) true true (* (Variables|Default|GetElevatorSpeed) 3.0) false)
                  (Variables|Default|SetCurrentHeight (+ (Variables|Default|GetCurrentHeight) (- (Variables|Default|GetStoryHeight) (Variables|Default|GetCurrentHeight))))
                  (Variables|Default|SetIsMoving false)
                  (Variables|Default|SetWhatFloorImOn 3)
                  (CallFunction|OpenDoors))))))))
    (:then_1
      ;[0 0.3627 1] OpenDoors
      (if (not (Variables|Default|GetJustOpened))
        (if (Math|Boolean|ORBoolean (== (Variables|Default|GetStaticMesh) Component) (== (Variables|Default|Getlift_door) Component) (== (Variables|Default|Getlift_door1) Component))
          (if (not (Variables|Default|GetIsMoving))
            (Variables|Default|SetIsMoving true)
            (Utilities|FlowControl|DoOnce false :!label _label
              (:Completed
                (Utilities|FlowControl|Sequence
                  (:then_0
                    (Components|MoveComponentTo _staticmesh_2 (Math|Vector|MakeVector (- (.x (.location _returnvalue_11)) 5e+01) (.y (.location _returnvalue_11)) (.z (.location _returnvalue_11))) (.rotation _returnvalue_11) true true 1.0 false))
                  (:then_1
                    (Components|MoveComponentTo _lift_door (Math|Vector|MakeVector (- (.x (.location _returnvalue_12)) 1e+02) (.y (.location _returnvalue_12)) (.z (.location _returnvalue_12))) (.rotation _returnvalue_12) true true 1.0 false))
                  (:then_2
                    (Components|MoveComponentTo _lift_door1 (Math|Vector|MakeVector (- (.x (.location _returnvalue_13)) 1.5e+02) (.y (.location _returnvalue_13)) (.z (.location _returnvalue_13))) (.rotation _returnvalue_13) true true 1.0 false)))
                (Variables|Default|SetIsMoving false)
                (Variables|Default|SetJustOpened true)
                (goto _label_2 Reset)))))))
    (:then_2
      ;[0 0.3627 1] CloseDoors
      (if (Variables|Default|GetJustOpened)
        (if (Math|Boolean|ORBoolean (== (Variables|Default|GetStaticMesh) Component) (== (Variables|Default|Getlift_door) Component) (== (Variables|Default|Getlift_door1) Component))
          (if (not (Variables|Default|GetIsMoving))
            (Variables|Default|SetIsMoving true)
            (Utilities|FlowControl|DoOnce false :!label _label_2
              (:Completed
                (Utilities|FlowControl|Sequence
                  (:then_0
                    (Components|MoveComponentTo _staticmesh (Math|Vector|MakeVector (+ (.x (.location _returnvalue_4)) 5e+01) (.y (.location _returnvalue_4)) (.z (.location _returnvalue_4))) (.rotation _returnvalue_4) true true 1.0 false))
                  (:then_1
                    (Components|MoveComponentTo _lift_door1_2 (Math|Vector|MakeVector (+ (.x (.location _returnvalue_5)) 1.5e+02) (.y (.location _returnvalue_5)) (.z (.location _returnvalue_5))) (.rotation _returnvalue_5) true true 1.0 false))
                  (:then_2
                    (Components|MoveComponentTo _lift_door_2 (Math|Vector|MakeVector (+ (.x (.location _returnvalue_3)) 1e+02) (.y (.location _returnvalue_3)) (.z (.location _returnvalue_3))) (.rotation _returnvalue_3) true true 1.0 false)))
                (Variables|Default|SetIsMoving false)
                (Variables|Default|SetJustOpened false)
                (goto _label Reset)))))))))

(event EventTick
  (params (DeltaSeconds :type Float%20%28single-precision%29))
  ;[0.9425 0.1353 1] LineTrace
  (bind _asbp_human (Utilities|Casting|CastToBP_Human (Components|GetOwner (Variables|/Script/HelloNeighbor.Human|GetCamera (Variables|Default|GetBP_Human))))))

(event Input|KeyboardEvents|E
  (params (Key :type Key%20Structure))
  (bind _bp_human (Variables|Default|GetBP_Human))
  (bind _camera (Variables|/Script/HelloNeighbor.Human|GetCamera _bp_human))
  (bind _returnvalue (Transformation|GetWorldLocation _camera))
  ;[0.9425 0.1353 1] LineTrace
  (:Pressed
    (Utilities|FlowControl|Sequence
      (:then_0
        (bind (_outhits _returnvalue_2) (Collision|MultiLineTraceByChannel _returnvalue (+ _returnvalue (* (Math|Vector|GetForwardVector _camera) 2e+02)) "TraceTypeQuery1" false (Utilities|Array|MakeArray (stale EventTick _asbp_human)) "None" false))
        (if _returnvalue_2
          (bind _asbp_my_elevator_2 (Utilities|Casting|CastToBP_MyElevator2 (.HitActor (Collision|BreakHitResult (Utilities|Array|Get(acopy) _outhits)))))
          (CallFunction|UpDown _asbp_my_elevator_2 (.HitComponent (Collision|BreakHitResult (Utilities|Array|Get(acopy) _outhits)))))))))

(fn ConstructionScript
  (Variables|Default|SetStoryHeight (* (Variables|Default|GetTheStoryHeight) (Variables|Default|GetMaxStories)))
  (if (> (Variables|Default|GetStoryHeight) (+ (Variables|Default|GetTheStoryHeight) 1.0))
    (Rendering|SetVisibility (Variables|Default|GetUpButton2) true false)
    (if (> (Variables|Default|GetStoryHeight) (+ (* (Variables|Default|GetTheStoryHeight) 2.0) 1.0))
      (Rendering|SetVisibility (Variables|Default|GetUpbuttoon3) true false))))