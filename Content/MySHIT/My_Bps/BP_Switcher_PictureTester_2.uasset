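; Toggle switch (tumbler) actor that animates a Switch component between open and closed and tracks an IsUnlocked flag.
; Action events and hits on the Switch reverse its moving state, and tumbler state changes also drive it while playing an on/off sound cue.
; Tick runs RotateSwitch, which pitches the component at a set speed, clamps it at its limits and then sets the tumbler state on or off.
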(event EventBeginPlay
  (bind _switch (Variables|Default|GetSwitch))
  ;[1 1 1] Comment
  (switch Utilities|FlowControl|Switch|SwitchonETumblerState (Class|Tumbler|GetTumblerState)
    (:TUMBLER_ON
      (Class|MovingComponent|SetMovingState _switch "MS_OPENING"))
    (:TUMBLER_OFF
      (Class|MovingComponent|SetMovingState _switch "MS_CLOSING"))))

(event Collision|EventHit
  (params (MyComp :type Primitive%20Component%20Object%20Reference) (Other :type Actor%20Object%20Reference) (OtherComp :type Primitive%20Component%20Object%20Reference) (bSelfMoved :type Boolean) (HitLocation :type Vector :default "0, 0, 0") (HitNormal :type Vector :default "0, 0, 0") (NormalImpulse :type Vector :default "0, 0, 0") (Hit :type Hit%20Result%20Structure%20%28by%20ref%29))
  (bind _switch (Variables|Default|GetSwitch))
  (if (== MyComp (Variables|Default|GetSwitch))
    (switch Utilities|FlowControl|Switch|SwitchonEMovingState (Class|MovingComponent|GetMovingState (Variables|Default|GetSwitch))
      (:MS_OPEN
        (Variables|Default|SetIsUnlocked true)
        (Class|MovingComponent|SetMovingState _switch "MS_CLOSING"))
      (:MS_CLOSE
        (Variables|Default|SetIsUnlocked false)
        (Class|MovingComponent|SetMovingState _switch "MS_OPENING"))
      (:MS_OPENING
        (Class|MovingComponent|SetMovingState _switch "MS_CLOSING"))
      (:MS_CLOSING
        (Class|MovingComponent|SetMovingState _switch "MS_OPENING")))))

(event EventTick
  (params (DeltaSeconds :type Float%20%28single-precision%29))
  ;[1 1 1] Comment
  (CallFunction|RotateSwitch DeltaSeconds))

(event EventOnChangeTumblerState
  (params (NewState :type ETumblerState%20Enum :default "TUMBLER_ON"))
  (bind _switch (Variables|Default|GetSwitch))
  ;[1 1 1] Comment
  (switch Utilities|FlowControl|Switch|SwitchonETumblerState NewState
    (:TUMBLER_ON
      (Class|MovingComponent|SetMovingState _switch "MS_OPENING"))
    (:TUMBLER_OFF
      (Class|MovingComponent|SetMovingState _switch "MS_CLOSING")))
  (Audio|Components|Audio|Play (Variables|Default|Geton_off_switch_Cue) 0.0))

(event EventOnEventAction
  (params (ActionMaker :type Actor%20Object%20Reference) (SpecialComponent :type Primitive%20Component%20Object%20Reference))
  (bind _switch (Variables|Default|GetSwitch))
  ;[1 1 1] Comment
  (if (== SpecialComponent (Variables|Default|GetSwitch))
    (switch Utilities|FlowControl|Switch|SwitchonEMovingState (Class|MovingComponent|GetMovingState (Variables|Default|GetSwitch))
      (:MS_OPEN
        (Variables|Default|SetIsUnlocked true)
        (Class|MovingComponent|SetMovingState _switch "MS_CLOSING"))
      (:MS_CLOSE
        (Variables|Default|SetIsUnlocked false)
        (Class|MovingComponent|SetMovingState _switch "MS_OPENING"))
      (:MS_OPENING
        (Variables|Default|SetIsUnlocked true)
        (Class|MovingComponent|SetMovingState _switch "MS_CLOSING"))
      (:MS_CLOSING
        (Variables|Default|SetIsUnlocked false)
        (Class|MovingComponent|SetMovingState _switch "MS_OPENING")))))

(fn ConstructionScript)

(fn RotateSwitch
  (params (DeltaTime :type Float%20%28single-precision%29))
  (bind _switch (Variables|Default|GetSwitch))
  (bind _switch_2 (Variables|Default|GetSwitch))
  (bind _speedswitch (Variables|Default|GetSpeedSwitch))
  (bind _returnvalue (* DeltaTime _speedswitch))
  (bind _relativerotation (Variables|/Script/Engine.SceneComponent|GetRelativeRotation _switch_2))
  (switch Utilities|FlowControl|Switch|SwitchonEMovingState (Class|MovingComponent|GetMovingState (Variables|Default|GetSwitch))
    (:MS_OPENING
      ;[1 1 1] Comment
      (Transformation|AddRelativeRotation _switch (Math|Rotator|MakeRotator 0.0 (* _returnvalue -1.0) 0.0) false false)
      (if (<= (.pitch (Variables|/Script/Engine.SceneComponent|GetRelativeRotation _switch)) (Variables|Default|GetMinRotateSwitch))
        (Transformation|SetRelativeRotation (Variables|Default|GetSwitch) (Math|Rotator|MakeRotator 0.0 (Variables|Default|GetMinRotateSwitch) 0.0) false false)
        (Class|MovingComponent|SetMovingState (Variables|Default|GetSwitch) "MS_OPEN")
        (Class|Tumbler|SetTumblerState "TUMBLER_ON")))
    (:MS_CLOSING
      ;[1 1 1] Comment
      (Transformation|AddRelativeRotation _switch_2 (Math|Rotator|MakeRotator 0.0 (* _returnvalue 1.0) 0.0) false false)
      (if (or (>= (.pitch _relativerotation) (Variables|Default|GetMaxRotateSwitch)) (< (.pitch _relativerotation) 0.0))
        (Transformation|SetRelativeRotation (Variables|Default|GetSwitch) (Math|Rotator|MakeRotator 0.0 (Variables|Default|GetMaxRotateSwitch) 0.0) false false)
        (Class|MovingComponent|SetMovingState (Variables|Default|GetSwitch) "MS_CLOSE")
        (Class|Tumbler|SetTumblerState "TUMBLER_OFF")))))

(fn OnIsActionComponent
  (params (Component :type Primitive%20Component%20Object%20Reference))
  (return true))