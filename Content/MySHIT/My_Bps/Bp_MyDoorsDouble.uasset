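; Double door actor that swings both leaves open and shut, launches humans it hits, and can balance a spawned bucket while closed.
; A Box overlap enables input and shifts BoundComponent vertically; E then traces from the camera to the hit door's MoveNewDoor, which flip-flops both leaves' yaw.
; The construction script poses MeshDoor by state, turns the arrow red on WorldStatic overlap and sets link data between two proxy points.
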(event OnComponentBeginOverlap(Box)
  (params (OverlappedComponent :type Primitive%20Component%20Object%20Reference) (OtherActor :type Actor%20Object%20Reference) (OtherComp :type Primitive%20Component%20Object%20Reference) (OtherBodyIndex :type Integer) (bFromSweep :type Boolean) (SweepResult :type Hit%20Result%20Structure%20%28by%20ref%29))
  (bind _boundcomponent (Variables|Default|GetBoundComponent))
  (bind _relativelocation (Variables|/Script/Engine.SceneComponent|GetRelativeLocation _boundcomponent))
  ;[1 1 1] MoveBox COmponent
  (Utilities|Casting|CastToBP_Human OtherActor)
  (Input|EnableInput (Game|GetPlayerController 0))
  (Variables|Default|SetIsIn true)
  (Components|MoveComponentTo _boundcomponent (Math|Vector|MakeVector (.x _relativelocation) (.y _relativelocation) (+ (.z _relativelocation) 4e+02)) (Variables|/Script/Engine.SceneComponent|GetRelativeRotation _boundcomponent) false false 0.2 false))

(event OnComponentHit(MeshDoor)
  (params (HitComponent :type Primitive%20Component%20Object%20Reference) (OtherActor :type Actor%20Object%20Reference) (OtherComp :type Primitive%20Component%20Object%20Reference) (NormalImpulse :type Vector :default "0, 0, 0") (Hit :type Hit%20Result%20Structure%20%28by%20ref%29))
  ;[1 1 1] Нужно отталкивать дверью игрока
  (if (Class|Door|IsCheckHit)
    (bind _ashuman (Utilities|Casting|CastToHuman OtherActor))
    (Character|LaunchCharacter _ashuman (* (Math|Vector|RotateVector (Variables|Default|Getm_vDirectionOpen) (Transformation|GetActorRotation)) (/ (Class|Door|GetCurrentForce) 1e+03)) false false)))

(event OnComponentHit(MeshDoor2)
  (params (HitComponent :type Primitive%20Component%20Object%20Reference) (OtherActor :type Actor%20Object%20Reference) (OtherComp :type Primitive%20Component%20Object%20Reference) (NormalImpulse :type Vector :default "0, 0, 0") (Hit :type Hit%20Result%20Structure%20%28by%20ref%29))
  (if (Class|Door|IsCheckHit)
    (bind _asbp_human (Utilities|Casting|CastToBP_Human OtherActor))
    (Character|LaunchCharacter _asbp_human (* (Math|Vector|RotateVector (Variables|Default|Getm_vDirectionOpen) (Transformation|GetActorRotation)) (/ (Class|Door|GetCurrentForce) 1e+03)) false false)))

(event OnComponentEndOverlap(Box)
  (params (OverlappedComponent :type Primitive%20Component%20Object%20Reference) (OtherActor :type Actor%20Object%20Reference) (OtherComp :type Primitive%20Component%20Object%20Reference) (OtherBodyIndex :type Integer))
  (bind _boundcomponent (Variables|Default|GetBoundComponent))
  (bind _relativelocation (Variables|/Script/Engine.SceneComponent|GetRelativeLocation _boundcomponent))
  ;[1 1 1] MoveBox COmponent
  (Utilities|Casting|CastToBP_Human OtherActor)
  (Input|DisableInput (Game|GetPlayerController 0))
  (Variables|Default|SetIsIn false)
  (Components|MoveComponentTo _boundcomponent (Math|Vector|MakeVector (.x _relativelocation) (.y _relativelocation) (- (.z _relativelocation) 4e+02)) (Variables|/Script/Engine.SceneComponent|GetRelativeRotation _boundcomponent) false false 0.2 false))

(event Custom|MoveNewDoor
  (params (Component :type Primitive%20Component%20Object%20Reference))
  (bind _isin (Variables|Default|GetIsIn))
  (bind _meshdoor (Variables|Default|GetMeshDoor))
  (bind _meshdoor2 (Variables|Default|GetMeshDoor2))
  (bind _relativelocation (Variables|/Script/Engine.SceneComponent|GetRelativeLocation _meshdoor))
  (bind _relativerotation (Variables|/Script/Engine.SceneComponent|GetRelativeRotation _meshdoor))
  (bind _relativerotation_2 (Variables|/Script/Engine.SceneComponent|GetRelativeRotation _meshdoor))
  (bind _relativelocation_2 (Variables|/Script/Engine.SceneComponent|GetRelativeLocation _meshdoor2))
  (bind _relativerotation_3 (Variables|/Script/Engine.SceneComponent|GetRelativeRotation _meshdoor2))
  ;[1 1 1] MoveDoor
  (Utilities|FlowControl|Sequence
    (:then_0
      (if (== Component (Variables|Default|GetMeshDoor2))
        (Utilities|FlowControl|Delay 0.2)
        (if _isin
          (Utilities|FlowControl|Sequence
            (:then_0
              (Utilities|FlowControl|FlipFlop :!label _label
                (:A
                  (Components|MoveComponentTo _meshdoor2 _relativelocation_2 (Math|Rotator|MakeRotator (.roll _relativerotation_3) (.pitch _relativerotation_3) (- (.yaw _relativerotation_3) 8e+01)) true true 0.3 false))
                (:B
                  (Components|MoveComponentTo _meshdoor2 _relativelocation_2 (Math|Rotator|MakeRotator (.roll _relativerotation_3) (.pitch _relativerotation_3) (+ (.yaw _relativerotation_3) 8e+01)) false false 0.3 false))))
            (:then_1
              (Utilities|FlowControl|FlipFlop :!label _label_2
                (:A
                  (Components|MoveComponentTo _meshdoor _relativelocation (Math|Rotator|MakeRotator (.roll _relativerotation) (.pitch _relativerotation) (+ (.yaw _relativerotation) 8e+01)) false false 0.2 false))
                (:B
                  (Components|MoveComponentTo _meshdoor _relativelocation (Math|Rotator|MakeRotator (.roll _relativerotation_2) (.pitch _relativerotation_2) (- (.yaw _relativerotation_2) 8e+01)) false false 0.2 false))))))))
    (:then_1
      (if (== Component (Variables|Default|GetMeshDoor))
        (if _isin
          (Utilities|FlowControl|Sequence
            (:then_0
              (goto _label_2))
            (:then_1
              (goto _label))))))))

(event EventOnForceChangeDoorState
  (params (NewState :type EDoorState%20Enum :default "DS_OPEN"))
  ;[1 1 1] Быстро изменить состояние двери
  (Default|CallEventChangeDoor NewState))

(event EventTick
  (params (DeltaSeconds :type Float%20%28single-precision%29))
  ;[1 1 1] Multine trace
  (Utilities|Casting|CastToBP_Human (Components|GetOwner (Variables|/Script/HelloNeighbor.Human|GetCamera (Variables|Default|GetBP_Human)))))

(event EventOnChangeDoorState
  (params (NewState :type EDoorState%20Enum :default "DS_OPEN"))
  ;[1 1 1] Изменили состояние двери
  (Default|CallEventChangeDoor NewState)
  (Utilities|FlowControl|FlipFlop
    (:A
      (CallFunction|MoveNewDoor))))

(event Input|KeyboardEvents|E
  (params (Key :type Key%20Structure))
  (bind _bp_human (Variables|Default|GetBP_Human))
  (bind _camera (Variables|/Script/HelloNeighbor.Human|GetCamera _bp_human))
  (bind _returnvalue (Transformation|GetWorldLocation _camera))
  (bind _returnvalue_2 (Math|Vector|GetForwardVector _camera))
  ;[1 1 1] Multine trace
  (:Pressed
    (bind (_outhits _returnvalue_3) (Collision|MultiLineTraceByChannel (+ (* _returnvalue_2 7e+01) _returnvalue) (+ _returnvalue (* _returnvalue_2 3e+02)) "TraceTypeQuery1" false 0 "Persistent" false))
    (if _returnvalue_3
      (bind _asbp_my_doors_double (Utilities|Casting|CastToBp_MyDoorsDouble (.HitActor (Collision|BreakHitResult (Utilities|Array|Get(acopy) _outhits)))))
      (CallFunction|MoveNewDoor _asbp_my_doors_double (.HitComponent (Collision|BreakHitResult (Utilities|Array|Get(acopy) _outhits)))))))

(event Input|KeyboardEvents|E
  (params (Key :type Key%20Structure))
  (:Pressed
    (CallFunction|MoveNewDoor)))

(fn ConstructionScript
  (bind _meshdoor (Variables|Default|GetMeshDoor))
  (bind _meshdoor_2 (Variables|Default|GetMeshDoor))
  (Components|Arrow|SetArrowColor(LinearColor) (Variables|Default|GetArrow) "(R=0.000000,G=1.000000,B=0.000000,A=1.000000)")
  (bind _outcomponents (Class|KismetSystemLibrary|ComponentOverlapComponents _meshdoor (Transformation|GetWorldTransform _meshdoor) (Utilities|Array|MakeArray "ObjectTypeQuery1") "/Script/Engine.ActorComponent" (Utilities|Array|MakeArray self)))
  (for _array_element _outcomponents
    (Development|PrintString (Utilities|GetDisplayName _array_element))
    (Components|Arrow|SetArrowColor(LinearColor) (Variables|Default|GetArrow) "(R=1.000000,G=0.000000,B=0.000000,A=1.000000)"))
  (Utilities|FlowControl|Sequence
    (:then_0
      (switch Utilities|FlowControl|Switch|SwitchonEDoorState (Class|Door|GetDoorState)
        (:DS_OPEN
          (Transformation|SetRelativeRotation _meshdoor_2 (Variables|Default|GetRotateOpen) false false))
        (:DS_CLOSE
          (Transformation|SetRelativeRotation _meshdoor_2 (Variables|Default|GetRotateClose) false false))))
    (:then_1
      (Class|Door|SetLinkData (Variables|/Script/Engine.SceneComponent|GetRelativeLocation (Variables|Default|GetLeftPointLinkProxy)) (Variables|/Script/Engine.SceneComponent|GetRelativeLocation (Variables|Default|GetRightPointLinkProxy))))))

(fn OnSetBucketonDoor
  (switch Utilities|FlowControl|Switch|SwitchonEDoorState (Class|Door|GetDoorState)
    (:DS_OPEN
      _)
    (:DS_CLOSING
      _)
    (:DS_CLOSE
      (Transformation|SetRelativeRotation (Variables|Default|GetMeshDoor) (Utilities|Plus (Variables|Default|GetRotateClose) (Variables|Default|GetBucketRotation)) false false)
      (bind _returnvalue (Game|SpawnActorfromClass "/Game/Objects/BP_Objects/BP_Bucket.BP_Bucket_C" (Transformation|GetActorTransform) "Undefined" 0 0))
      (Class|Actor|AddActorLocalTransform _returnvalue (Variables|Default|GetBucketTransform) false false)
      (Physics|SetSimulatePhysics (Variables|/Script/HelloNeighbor.Bucket|GetStaticMeshComponent _returnvalue) false)
      (Physics|SetSimulatePhysics (Variables|/Script/HelloNeighbor.Bucket|GetStaticMeshComponent _returnvalue) true))
    (:DS_OPENING
      _))
  (return _returnvalue))

(fn OnIsActionComponent
  (params (Component :type Primitive%20Component%20Object%20Reference))
  (return (or (== Component (Variables|Default|GetMeshDoor2)) (== Component (Variables|Default|GetMeshDoor)))))