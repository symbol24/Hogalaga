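; Trigger-driven random movie picker that rolls titles on a text component while a BP_Human is inside its trigger.
; Overlap lets Tick fire StartTimer up to 30 times through a DoN, and a self-rescheduling timer with growing delay slows the shuffle like a slot machine.
; Once the delay passes its limit, the text changes color and eases upward.
; Leaving the trigger hides the text and resets the delay and DoN.
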(event OnComponentEndOverlap(Trigger)
  (params (OverlappedComponent :type Primitive%20Component%20Object%20Reference) (OtherActor :type Actor%20Object%20Reference) (OtherComp :type Primitive%20Component%20Object%20Reference) (OtherBodyIndex :type Integer))
  ;[1 1 1] Remove Text
  (Utilities|Casting|CastToBP_Human OtherActor)
  (Variables|Default|SetWas%20Hit false)
  (Rendering|SetVisibility (Variables|Default|GetText) false false)
  (Variables|Default|SetDelay 0.0)
  (Variables|Default|SetHasStarted false)
  (CallFunction|ResetTimer))

(event OnComponentBeginOverlap(Trigger)
  (params (OverlappedComponent :type Primitive%20Component%20Object%20Reference) (OtherActor :type Actor%20Object%20Reference) (OtherComp :type Primitive%20Component%20Object%20Reference) (OtherBodyIndex :type Integer) (bFromSweep :type Boolean) (SweepResult :type Hit%20Result%20Structure%20%28by%20ref%29))
  (bind _text (Variables|Default|GetText))
  (bind _relativelocation (Variables|/Script/Engine.SceneComponent|GetRelativeLocation _text))
  (Utilities|Casting|CastToBP_Human OtherActor)
  (Variables|Default|SetWas%20Hit true)
  (if (Variables|Default|GetHasStarted)
    (Variables|Default|SetDelay (+ (Variables|Default|GetDelay) 0.01))
    (if (<= (Variables|Default|GetDelay) 0.5)
      (Utilities|Time|SetTimerbyEvent (delegate Custom|StartTimer) (Variables|Default|GetDelay))
      (else
        (Rendering|Components|TextRender|SetTextRenderColor (Variables|Default|GetText) (Variables|Default|GetNewVar_0))
        (Components|MoveComponentTo _text (Math|Vector|MakeVector (.x _relativelocation) (.y _relativelocation) (+ (.z _relativelocation) 5e+01)) (Variables|/Script/Engine.SceneComponent|GetRelativeRotation _text) true true 1.0 false)))))

(event Custom|StartTimer
  (bind _text (Variables|Default|GetText))
  (bind _relativelocation (Variables|/Script/Engine.SceneComponent|GetRelativeLocation _text))
  (CallFunction|GetRandomText)
  (Variables|Default|SetDelay (+ (Variables|Default|GetDelay) 0.01))
  (if (<= (Variables|Default|GetDelay) 0.5)
    (Utilities|Time|SetTimerbyEvent (delegate Custom|StartTimer) (Variables|Default|GetDelay))
    (else
      (Rendering|Components|TextRender|SetTextRenderColor (Variables|Default|GetText) (Variables|Default|GetNewVar_0))
      (Components|MoveComponentTo _text (Math|Vector|MakeVector (.x _relativelocation) (.y _relativelocation) (+ (.z _relativelocation) 5e+01)) (Variables|/Script/Engine.SceneComponent|GetRelativeRotation _text) true true 1.0 false))))

(event Custom|ResetTimer
  (Utilities|FlowControl|DoN 30) ; enters at Reset
)

(event EventTick
  (params (DeltaSeconds :type Float%20%28single-precision%29))
  (if (Variables|Default|GetWas%20Hit)
    (Utilities|FlowControl|DoN 30
      (:Exit
        (CallFunction|StartTimer)
        (Variables|Default|SetHasStarted true)))))

(fn ConstructionScript)

(fn GetRandomText
  (bind _movies (Variables|Default|GetMOVIES))
  (bind _returnvalue (Utilities|Array|Length _movies))
  (bind _returnvalue_2 (- _returnvalue 1))
  (bind _returnvalue_3 (Math|Random|RandomIntegerinRange 0 _returnvalue_2))
  (bind _output (Utilities|Array|Get(acopy) _movies _returnvalue_3))
  (bind _returnvalue_4 (Utilities|Text|ToText(String) _output))
  (Rendering|SetVisibility (Variables|Default|GetText) true false)
  (Rendering|Components|TextRender|SetText (Variables|Default|GetText) _returnvalue_4)
  (return (Utilities|String|ToString(Text) _returnvalue_4)))