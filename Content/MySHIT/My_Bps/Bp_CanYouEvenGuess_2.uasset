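; Configurable door actor that swings open on a yaw timeline, with mesh and material set from variables.
; Every Tick it polls a book key's pickup state and three switch actors' tumbler states, each playing or reversing the same timeline in sequence, so later checks can override earlier ones.
; Reversing only happens when ReverseDoor is set, and OnOffSwitc inverts the response to the Switcher2 switch.
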(event Custom|OpenDoor)

(event EventBeginPlay
  (Rendering|Material|SetMaterial (Variables|Default|GetStaticMesh) 0 (Variables|Default|GetMaterial)))

(event Collision|EventActorBeginOverlap
  (params (OtherActor :type Actor%20Object%20Reference)))

(event EventTick
  (params (DeltaSeconds :type Float%20%28single-precision%29))
  (bind _onoffswitc (Variables|Default|GetOnOffSwitc))
  (Utilities|FlowControl|Sequence
    (:then_0
      (bind _asbp_my_book_key (Utilities|Casting|CastToBP_MyBookKey (Components|GetOwner (Variables|/Script/HelloNeighbor.FlatActor|GetFlatComponent (Variables|Default|GetTheBook)))))
      (bind _output_get (Variables|Default|SetbInCubeHasPickedUp (Variables|/Hogalaga/MySHIT/My_Bps/BP_MyBookKey.BP_MyBookKey_C|GetHaspickedUp _asbp_my_book_key)))
      (if _output_get
        (bind _newtrack_0 (Timeline|MoveDoor Play)
          (:Update
            (Transformation|SetRelativeRotation (Variables|Debug|GetStaticMeshComponent) (Math|Rotator|MakeRotator 0.0 0.0 _newtrack_0) false false)))
        (else
          (if (Variables|Default|GetReverseDoor?) :!label _label
            (Timeline|MoveDoor Reverse)))))
    (:then_1
      (bind _asbp_switcher_picture_tester (Utilities|Casting|CastToBP_Switcher_PictureTester (Components|GetOwner (Variables|/Script/HelloNeighbor.FlatActor|GetFlatComponent (Variables|Default|GetPictureSwitcherTester)))))
      (if (Utilities|Enum|Equal(Enum) (Variables|/Script/HelloNeighbor.Tumbler|Getm_eState _asbp_switcher_picture_tester) "TUMBLER_ON")
        (Timeline|MoveDoor Play)
        (else
          (goto _label))))
    (:then_2
      (bind _asbp_switcher_picture (Utilities|Casting|CastToBP_Switcher_Picture (Components|GetOwner (Variables|/Script/HelloNeighbor.FlatActor|GetFlatComponent (Variables|Default|GetSwitcher_Picture)))))
      (if (Utilities|Enum|Equal(Enum) (Variables|/Script/HelloNeighbor.Tumbler|Getm_eState _asbp_switcher_picture) "TUMBLER_ON")
        (Timeline|MoveDoor Play)
        (else
          (goto _label))))
    (:then_3
      (bind _asbp_switcher_2 (Utilities|Casting|CastToBP_Switcher_2 (Components|GetOwner (Variables|/Script/HelloNeighbor.FlatActor|GetFlatComponent (Variables|Default|GetSwitcher_2)))))
      (if (Utilities|Enum|Equal(Enum) (Variables|/Script/HelloNeighbor.Tumbler|Getm_eState _asbp_switcher_2) "TUMBLER_ON")
        (if _onoffswitc
          (goto _label)
          (else
            (Timeline|MoveDoor Play)))
        (elif _onoffswitc
          (Timeline|MoveDoor Play)
          (else
            (goto _label)))))))

(fn ConstructionScript
  (bind _staticmesh (Variables|Default|GetStaticMesh))
  (Components|StaticMesh|SetStaticMesh _staticmesh (Variables|Default|GetActualStaticMesh))
  (Rendering|Material|SetMaterial _staticmesh 0 (Variables|Default|GetMaterial)))