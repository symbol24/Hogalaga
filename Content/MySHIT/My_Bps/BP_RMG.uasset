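; BP_RMG is a random movie picker that displays an entry from its MOVIES array when a BP_Human enters its trigger.
; On begin overlap it makes the Text component visible and sets it to the element at a random index from zero to AmountOfMovies, inclusive.
; On end overlap by a BP_Human it hides the text again, so each entry draws a new pick.
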(event OnComponentBeginOverlap(Trigger)
  (params (OverlappedComponent :type Primitive%20Component%20Object%20Reference) (OtherActor :type Actor%20Object%20Reference) (OtherComp :type Primitive%20Component%20Object%20Reference) (OtherBodyIndex :type Integer) (bFromSweep :type Boolean) (SweepResult :type Hit%20Result%20Structure%20%28by%20ref%29))
  ;[1 1 1] RNG Trigger and Set Visibility of Text
  (Utilities|Casting|CastToBP_Human OtherActor)
  (Rendering|SetVisibility (Variables|Default|GetText) true false)
  (Rendering|Components|TextRender|SetText (Variables|Default|GetText) (Utilities|Text|ToText(String) (Utilities|Array|Get(acopy) (Variables|Default|GetMOVIES) (Math|Random|RandomIntegerinRange 0 (Variables|Default|GetAmountOfMovies))))))

(event OnComponentEndOverlap(Trigger)
  (params (OverlappedComponent :type Primitive%20Component%20Object%20Reference) (OtherActor :type Actor%20Object%20Reference) (OtherComp :type Primitive%20Component%20Object%20Reference) (OtherBodyIndex :type Integer))
  ;[1 1 1] Remove Text
  (Utilities|Casting|CastToBP_Human OtherActor)
  (Rendering|SetVisibility (Variables|Default|GetText) false false))

(fn ConstructionScript)