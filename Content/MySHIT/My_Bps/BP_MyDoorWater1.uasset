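; Interactive physics door that can be tied to a WaterBlock, clearing its block if locked when draining ends.
; Using the door toggles its state, briefly firing open or close thrusters on the simulated mesh.
; Tick checks the rotation after a short delay, then snaps to the start or end limit and stops physics.
; A closed door can also be set slightly rotated with a spawned physics bucket on it.
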(event Custom|OnEndDrain
  (if (Class|Door|IsLock)
    (Class|Door|SetBlock false)))

(event EventBeginPlay
  (bind _waterblock (Variables|Default|GetWaterBlock))
  ;[1 1 1] Comment
  (Variables|Default|SetEnd (Utilities|Plus (Variables|/Script/Engine.SceneComponent|GetRelativeRotation (Variables|Default|GetDoor)) (Variables|Default|GetEnd)))
  (Variables|Default|SetStart (Utilities|Plus (Variables|/Script/Engine.SceneComponent|GetRelativeRotation (Variables|Default|GetDoor)) (Variables|Default|GetStart)))
  (Physics|SetSimulatePhysics (Variables|Default|GetDoor) false)
  (if (Utilities|IsValid _waterblock)
    (EventDispatchers|AssignOnEndDrain _waterblock (delegate Custom|OnEndDrain))))

(event EventOnForceChangeDoorState
  (params (NewState :type EDoorState%20Enum :default "DS_OPEN"))
  ;[1 1 1] Comment
  (switch Utilities|FlowControl|Switch|SwitchonEDoorState NewState
    (:DS_OPEN
      (Transformation|SetRelativeRotation (Variables|Default|GetDoor) (Variables|Default|GetEnd) false false))
    (:DS_CLOSE
      (Transformation|SetRelativeRotation (Variables|Default|GetDoor) (Variables|Default|GetStart) false false))))

(event EventTick
  (params (DeltaSeconds :type Float%20%28single-precision%29))
  ;[1 1 1] Comment
  (CallFunction|CheckDoor DeltaSeconds))

(event EventOnEventAction
  (params (ActionMaker :type Actor%20Object%20Reference) (SpecialComponent :type Primitive%20Component%20Object%20Reference))
  ;[1 1 1] Comment
  (if (== SpecialComponent (Variables|Default|GetDoor))
    (bind _ascharacter (Utilities|Casting|CastToCharacter ActionMaker))
    (switch Utilities|FlowControl|Switch|SwitchonEDoorState (Class|Door|GetDoorState)
      (:DS_OPEN
        (Class|Door|SetDoorState "DS_CLOSING" _ascharacter 0.0 :!label _label))
      (:DS_CLOSING
        (Class|Door|SetDoorState "DS_OPENING" _ascharacter 0.0 :!label _label_2))
      (:DS_CLOSE
        (goto _label_2))
      (:DS_OPENING
        (goto _label)))
    (Variables|Default|SetTimer 0.0)))

(event EventOnChangeDoorState
  (params (NewState :type EDoorState%20Enum :default "DS_OPEN"))
  (bind _returnvalue (Class|Door|GetCurrentForce))
  (bind _physicsthrusteropen (Variables|Default|GetPhysicsThrusterOpen))
  (bind _physicsthrusterclose (Variables|Default|GetPhysicsThrusterClose))
  ;[1 1 1] Comment
  (switch Utilities|FlowControl|Switch|SwitchonEDoorState NewState
    (:DS_CLOSING
      (Physics|SetSimulatePhysics (Variables|Default|GetDoor) true)
      (Variables|/Script/Engine.PhysicsThrusterComponent|SetThrustStrength _physicsthrusterclose _returnvalue)
      (Components|Activation|Activate _physicsthrusterclose false)
      (Utilities|FlowControl|Delay 0.2)
      (Components|Activation|Deactivate (Variables|Default|GetPhysicsThrusterClose)))
    (:DS_OPENING
      (Physics|SetSimulatePhysics (Variables|Default|GetDoor) true)
      (Variables|/Script/Engine.PhysicsThrusterComponent|SetThrustStrength _physicsthrusteropen (* _returnvalue 2.0))
      (Components|Activation|Activate _physicsthrusteropen false)
      (Utilities|FlowControl|Delay 0.2)
      (Components|Activation|Deactivate (Variables|Default|GetPhysicsThrusterOpen)))))

(fn ConstructionScript)

(fn CheckDoor
  (params (DeltaTime :type Float%20%28single-precision%29))
  (bind _door (Variables|Default|GetDoor))
  (bind _relativerotation (Variables|/Script/Engine.SceneComponent|GetRelativeRotation _door))
  (switch Utilities|FlowControl|Switch|SwitchonEDoorState (Class|Door|GetDoorState)
    (:DS_CLOSING
      _)
    (:DS_OPENING
      _))
  (bind _output_get (Variables|Default|SetTimer (+ DeltaTime (Variables|Default|GetTimer))))
  (if (> _output_get 0.5)
    (if (Math|Rotator|Equal(Rotator) (Variables|Default|GetEnd) _relativerotation 5.0)
      (Class|Door|SetDoorState "DS_OPEN" 0 0.0)
      (Transformation|SetRelativeRotation (Variables|Default|GetDoor) (Variables|Default|GetEnd) false false)
      (Physics|SetSimulatePhysics (Variables|Default|GetDoor) false)
      (Physics|SetSimulatePhysics (Variables|Default|GetDoor) false)
      (Variables|Default|SetTimer 0.0 :!label _label)
      (elif (Math|Rotator|Equal(Rotator) _relativerotation (Variables|Default|GetStart) 2.0)
        (Class|Door|SetDoorState "DS_CLOSE" 0 0.0)
        (Transformation|SetRelativeRotation (Variables|Default|GetDoor) (Variables|Default|GetStart) false false)
        (Physics|SetSimulatePhysics (Variables|Default|GetDoor) false)
        (goto _label)))))

(fn OnSetBucketonDoor
  (switch Utilities|FlowControl|Switch|SwitchonEDoorState (Class|Door|GetDoorState)
    (:DS_OPEN
      _)
    (:DS_CLOSING
      _)
    (:DS_CLOSE
      (Transformation|SetRelativeRotation (Variables|Default|GetDoor) (Utilities|Plus (Variables|Default|GetStart) (Variables|Default|GetDoorRotationForBucket)) false false)
      (bind _returnvalue (Game|SpawnActorfromClass "/Game/Objects/BP_Objects/BP_Bucket.BP_Bucket_C" (Transformation|GetActorTransform) "Undefined" 0 0))
      (Class|Actor|AddActorLocalTransform _returnvalue (Variables|Default|GetBucketTransform) false false)
      (Physics|SetSimulatePhysics (Variables|/Script/HelloNeighbor.Bucket|GetStaticMeshComponent _returnvalue) false)
      (Physics|SetSimulatePhysics (Variables|/Script/HelloNeighbor.Bucket|GetStaticMeshComponent _returnvalue) true))
    (:DS_OPENING
      _))
  (return _returnvalue))

(fn OnIsActionComponent
  (params (Component :type Primitive%20Component%20Object%20Reference))
  (return (== Component (Variables|Default|GetDoor))))