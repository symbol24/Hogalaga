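; Double-door actor that the player opens and closes by pressing input inside its trigger box while aiming at either leaf.
; A camera trace calls DoorLogic to toggle the inherited door state, whose change event swings only MeshDoor2 by relative yaw.
; Door hits can launch characters, and a bucket can be spawned on the closed door.
; The construction script flags static overlaps via arrow color, poses MeshDoor and sets link data.
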(event OnComponentBeginOverlap(Box)
  (params (OverlappedComponent :type Primitive%20Component%20Object%20Reference) (OtherActor :type Actor%20Object%20Reference) (OtherComp :type Primitive%20Component%20Object%20Reference) (OtherBodyIndex :type Integer) (bFromSweep :type Boolean) (SweepResult :type Hit%20Result%20Structure%20%28by%20ref%29))
  ;[1 1 1] MoveBox COmponent
  (Utilities|Casting|CastToBP_Human OtherActor)
  (Input|EnableInput (Game|GetPlayerController 0))
  (Variables|Default|SetIsIn true))

(event OnComponentHit(MeshDoor)
  (params (HitComponent :type Primitive%20Component%20Object%20Reference) (OtherActor :type Actor%20Object%20Reference) (OtherComp :type Primitive%20Component%20Object%20Reference) (NormalImpulse :type Vector :default "0, 0, 0") (Hit :type Hit%20Result%20Structure%20%28by%20ref%29))
  ;[1 1 1] Нужно отталкивать дверью игрока
  (if (Class|Door|IsCheckHit)
    (bind _ashuman (Utilities|Casting|CastToHuman OtherActor))
    (Character|LaunchCharacter _ashuman (* (Math|Vector|RotateVector (Variables|Default|Getm_vDirectionOpen) (Transformation|GetActorRotation)) (/ (Class|Door|GetCurrentForce) 1e+03)) false false)))

(event OnComponentHit(MeshDoor2)
  (params (HitComponent :type Primitive%20Component%20Object%20Reference) (OtherActor :type Actor%20Object%20Reference) (OtherComp :type Primitive%20Component%20Object%20Reference) (NormalImpulse :type Vector :default "0, 0, 0") (Hit :type Hit%20Result%20Structure%20%28by%20ref%29))
  ;[1 1 1] What
  (if (Class|Door|IsCheckHit)
    (bind _asbp_human (Utilities|Casting|CastToBP_Human OtherActor))
    (Character|LaunchCharacter _asbp_human (* (Math|Vector|RotateVector (Variables|Default|Getm_vDirectionOpen) (Transformation|GetActorRotation)) (/ (Class|Door|GetCurrentForce) 1e+03)) false false)))

(event OnComponentEndOverlap(Box)
  (params (OverlappedComponent :type Primitive%20Component%20Object%20Reference) (OtherActor :type Actor%20Object%20Reference) (OtherComp :type Primitive%20Component%20Object%20Reference) (OtherBodyIndex :type Integer))
  ;[1 1 1] MoveBox COmponent
  (Utilities|Casting|CastToBP_Human OtherActor)
  (Input|DisableInput (Game|GetPlayerController 0))
  (Variables|Default|SetIsIn false))

(event Custom|MoveNewDoor
  (params (Component :type Primitive%20Component%20Object%20Reference))
  ;[1 1 1] HitDoor
  (if (or (== Component (Variables|Default|GetMeshDoor2)) (== Component (Variables|Default|GetMeshDoor)))
    (CallFunction|DoorLogic)))

(event Custom|Flip1
  (bind _meshdoor2 (Variables|Default|GetMeshDoor2))
  (bind _relativerotation (Variables|/Script/Engine.SceneComponent|GetRelativeRotation _meshdoor2))
  ;[1 1 1] MoveDoor
  ;;[1 1 1] Flip01
  (Utilities|FlowControl|DoOnce false :!label _label
    (:Completed
      (Components|MoveComponentTo _meshdoor2 (Variables|/Script/Engine.SceneComponent|GetRelativeLocation _meshdoor2) (Math|Rotator|MakeRotator (.roll _relativerotation) (.pitch _relativerotation) (- (.yaw _relativerotation) 8e+01)) true true 0.3 false)
      (Utilities|FlowControl|Delay 0.5)
      (Variables|Default|SetIsMoving false)
      (goto _label Reset))))

(event Custom|Flop1
  (bind _meshdoor2 (Variables|Default|GetMeshDoor2))
  (bind _relativerotation (Variables|/Script/Engine.SceneComponent|GetRelativeRotation _meshdoor2))
  ;[1 1 1] MoveDoor
  ;;[1 1 1] Flop-01
  (Utilities|FlowControl|DoOnce false :!label _label
    (:Completed
      (Components|MoveComponentTo _meshdoor2 (Variables|/Script/Engine.SceneComponent|GetRelativeLocation _meshdoor2) (Math|Rotator|MakeRotator (.roll _relativerotation) (.pitch _relativerotation) (+ (.yaw _relativerotation) 8e+01)) false false 0.3 false)
      (Utilities|FlowControl|Delay 0.5)
      (Variables|Default|SetIsMoving false)
      (goto _label Reset))))

(event Custom|DoorLogic
  ;[1 1 1] DoorLogic States
  (Utilities|FlowControl|Sequence
    (:then_0
      (if (Utilities|Enum|Equal(Enum) (stale EventOnChangeDoorState NewState) "DS_OPEN")
        (Class|Door|SetDoorState "DS_CLOSING" 0 0.0)))
    (:then_1
      (if (Utilities|Enum|Equal(Enum) (stale EventOnChangeDoorState NewState) "DS_CLOSE")
        (Class|Door|SetDoorState "DS_OPENING" 0 0.0)))))

(event EventOnForceChangeDoorState
  (params (NewState :type EDoorState%20Enum :default "DS_OPEN"))
  ;[1 1 1] Быстро изменить состояние двери
  (Default|CallEventChangeDoor NewState))

(event EventBeginPlay
  ;[1 1 1] BeginPlayASSHOLE
  (Class|Door|SetDoorState "DS_CLOSING" 0 0.0)
  (Variables|Default|SetGamePlayedOnces true))

(event EventTick
  (params (DeltaSeconds :type Float%20%28single-precision%29))
  ;[1 1 1] Multine trace
  (bind _asbp_human (Utilities|Casting|CastToBP_Human (Components|GetOwner (Variables|/Script/HelloNeighbor.Human|GetCamera (Variables|Default|GetBP_Human))))))

(event EventOnChangeDoorState
  (params (NewState :type EDoorState%20Enum :default "DS_OPEN"))
  ;[1 1 1] Изменили состояние двери
  (Default|CallEventChangeDoor NewState)
  (switch Utilities|FlowControl|Switch|SwitchonEDoorState NewState
    (:DS_CLOSING
      (if (Variables|Default|GetIsOpened)
        (if (Variables|Default|GetGamePlayedOnces)
          (CallFunction|Flop1)
          (Variables|Default|SetIsOpened false))))
    (:DS_OPENING
      (if (not (Variables|Default|GetIsOpened))
        (CallFunction|Flip1)
        (Variables|Default|SetIsOpened true)))))

(event Input|ActionEvents|InputActionInputAction
  (params (Key :type Key%20Structure))
  (bind _bp_human (Variables|Default|GetBP_Human))
  (bind _camera (Variables|/Script/HelloNeighbor.Human|GetCamera _bp_human))
  (bind _returnvalue (Transformation|GetWorldLocation _camera))
  (bind _returnvalue_2 (Math|Vector|GetForwardVector _camera))
  ;[1 1 1] Multine trace
  (:Pressed
    (bind (_outhits _returnvalue_3) (Collision|MultiLineTraceByChannel (+ (* _returnvalue_2 7e+01) _returnvalue) (+ _returnvalue (* _returnvalue_2 3e+02)) "TraceTypeQuery1" false (Utilities|Array|MakeArray (stale EventTick _asbp_human)) "None" false))
    (if _returnvalue_3
      (bind _asbp_my_doors_double_vr_0_2 (Utilities|Casting|CastToBp_MyDoorsDoubleVr0_2 (.HitActor (Collision|BreakHitResult (Utilities|Array|Get(acopy) _outhits)))))
      (CallFunction|MoveNewDoor _asbp_my_doors_double_vr_0_2 (.HitComponent (Collision|BreakHitResult (Utilities|Array|Get(acopy) _outhits)))))))

(fn ConstructionScript
  (bind _meshdoor (Variables|Default|GetMeshDoor))
  (bind _meshdoor_2 (Variables|Default|GetMeshDoor))
  (Components|Arrow|SetArrowColor(LinearColor) (Variables|Default|GetArrow) "(R=0.000000,G=1.000000,B=0.000000,A=1.000000)")
  (bind _outcomponents (Class|KismetSystemLibrary|ComponentOverlapComponents _meshdoor (Transformation|GetWorldTransform _meshdoor) (Utilities|Array|MakeArray "ObjectTypeQuery1") "/Script/Engine.ActorComponent" (Utilities|Array|MakeArray self)))
  (for _array_element _outcomponents
    (Development|PrintString (Utilities|GetDisplayName _array_element))
    (Components|Arrow|SetArrowColor(LinearColor) (Variables|Default|GetArrow) "(R=1.000000,G=0.000000,B=0.000000,A=1.000000)"))
  (Utilities|FlowControl|Sequence
    (:then_0
      (switch Utilities|FlowControl|Switch|SwitchonEDoorState (Class|Door|GetDoorState)
        (:DS_OPEN
          (Transformation|SetRelativeRotation _meshdoor_2 (Variables|Default|GetRotateOpen) false false))
        (:DS_CLOSE
          (Transformation|SetRelativeRotation _meshdoor_2 (Variables|Default|GetRotateClose) false false))))
    (:then_1
      (Class|Door|SetLinkData (Variables|/Script/Engine.SceneComponent|GetRelativeLocation (Variables|Default|GetLeftPointLinkProxy)) (Variables|/Script/Engine.SceneComponent|GetRelativeLocation (Variables|Default|GetRightPointLinkProxy))))))

(fn OnSetBucketonDoor
  (switch Utilities|FlowControl|Switch|SwitchonEDoorState (Class|Door|GetDoorState)
    (:DS_OPEN
      _)
    (:DS_CLOSING
      _)
    (:DS_CLOSE
      (Transformation|SetRelativeRotation (Variables|Default|GetMeshDoor) (Utilities|Plus (Variables|Default|GetRotateClose) (Variables|Default|GetBucketRotation)) false false)
      (bind _returnvalue (Game|SpawnActorfromClass "/Game/Objects/BP_Objects/BP_Bucket.BP_Bucket_C" (Transformation|GetActorTransform) "Undefined" 0 0))
      (Class|Actor|AddActorLocalTransform _returnvalue (Variables|Default|GetBucketTransform) false false)
      (Physics|SetSimulatePhysics (Variables|/Script/HelloNeighbor.Bucket|GetStaticMeshComponent _returnvalue) false)
      (Physics|SetSimulatePhysics (Variables|/Script/HelloNeighbor.Bucket|GetStaticMeshComponent _returnvalue) true))
    (:DS_OPENING
      _))
  (return _returnvalue))

(fn OnIsActionComponent
  (params (Component :type Primitive%20Component%20Object%20Reference))
  (return (or (== Component (Variables|Default|GetMeshDoor)) (== Component (Variables|Default|GetMeshDoor2)))))