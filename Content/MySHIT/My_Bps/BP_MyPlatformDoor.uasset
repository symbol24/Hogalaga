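; BP_MyPlatformDoor is a door that drives a Platform component open or closed from electrical power and bookcase locks.
; On load, begin play and connection changes it opens when powered and closes when unpowered.
; Every Tick it also sets opening or closing from the MoveDoor flags of BookCaseLock and the TheBookLock array, regardless of power.
; Platform state changes play OpenClose while moving and stop it at either end.
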(event OnChangeMovingState(Platform)
  (params (NewState :type EMovingState%20Enum :default "MS_OPEN"))
  (bind _open_close (Variables|Default|GetOpen/Close))
  (switch Utilities|FlowControl|Switch|SwitchonEMovingState NewState
    (:MS_OPEN
      (Audio|Components|Audio|Stop _open_close :!label _label))
    (:MS_CLOSE
      (goto _label))
    (:MS_OPENING
      (Audio|Components|Audio|Play _open_close 0.0 :!label _label_2))
    (:MS_CLOSING
      (goto _label_2))))

(event EventOnChangeConnection
  (bind _platform (Variables|Default|GetPlatform))
  (bind _returnvalue (Class|MovingComponent|GetMovingState _platform))
  (if (Class|Electric|HasElectricity)
    (switch Utilities|FlowControl|Switch|SwitchonEMovingState _returnvalue
      (:MS_CLOSE
        _)
      (:MS_CLOSING
        _))
    (Class|MovingComponent|SetMovingState (Variables|Default|GetPlatform) "MS_OPENING")
    (else
      (switch Utilities|FlowControl|Switch|SwitchonEMovingState _returnvalue
        (:MS_OPEN
          _)
        (:MS_OPENING
          _))
      (Class|MovingComponent|SetMovingState (Variables|Default|GetPlatform) "MS_CLOSING"))))

(event EventBeginPlay
  (bind _platform (Variables|Default|GetPlatform))
  (bind _returnvalue (Class|MovingComponent|GetMovingState _platform))
  (if (Class|Electric|HasElectricity)
    (switch Utilities|FlowControl|Switch|SwitchonEMovingState _returnvalue
      (:MS_CLOSE
        _)
      (:MS_CLOSING
        _))
    (Class|MovingComponent|SetMovingState (Variables|Default|GetPlatform) "MS_OPENING")
    (else
      (switch Utilities|FlowControl|Switch|SwitchonEMovingState _returnvalue
        (:MS_OPEN
          _)
        (:MS_OPENING
          _))
      (Class|MovingComponent|SetMovingState (Variables|Default|GetPlatform) "MS_CLOSING"))))

(event EventTick
  (params (DeltaSeconds :type Float%20%28single-precision%29))
  (bind _platform (Variables|Default|GetPlatform))
  (Utilities|FlowControl|Sequence
    (:then_0
      (bind _asbp_my_bookcase_lock (Utilities|Casting|CastToBP_MyBookcaseLock (Components|GetOwner (Variables|/Script/HelloNeighbor.FlatActor|GetFlatComponent (Variables|Default|GetBookCaseLock)))))
      (if (Variables|/Hogalaga/MySHIT/My_Bps/BP_MyBookcaseLock.BP_MyBookcaseLock_C|GetMoveDoor _asbp_my_bookcase_lock)
        (Class|MovingComponent|SetMovingState _platform "MS_OPENING" :!label _label)
        (else
          (Class|MovingComponent|SetMovingState _platform "MS_CLOSING" :!label _label_2))))
    (:then_1
      (for _array_element (Variables|Default|GetTheBookLock)
        (if (Variables|/Hogalaga/MySHIT/My_Bps/BP_MyBookcaseLock.BP_MyBookcaseLock_C|GetMoveDoor _array_element)
          (bind _output_get (Variables|Default|SetIsTrue true))
          (if _output_get
            (goto _label))
          (elif (Variables|Default|GetIsTrue)
            (Variables|Default|SetIsTrue false)
            (else
              (goto _label_2))))))))

(event EventOnPostLoad
  (bind _platform (Variables|Default|GetPlatform))
  (bind _returnvalue (Class|MovingComponent|GetMovingState _platform))
  (if (Class|Electric|HasElectricity)
    (switch Utilities|FlowControl|Switch|SwitchonEMovingState _returnvalue
      (:MS_CLOSE
        _)
      (:MS_CLOSING
        _))
    (Class|MovingComponent|SetMovingState (Variables|Default|GetPlatform) "MS_OPENING")
    (else
      (switch Utilities|FlowControl|Switch|SwitchonEMovingState _returnvalue
        (:MS_OPEN
          _)
        (:MS_OPENING
          _))
      (Class|MovingComponent|SetMovingState (Variables|Default|GetPlatform) "MS_CLOSING"))))

(fn ConstructionScript)