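; Bookcase lock actor that flags a door to move when an accepted book key is in its trigger.
; Trigger overlaps track whether a BP_MyBookKey listed in BookKey0 is inside.
; Tick sets MoveDoor once that key has been picked up and its FlatComponent is Free, clearing it after a short delay while no key is registered.
; OnIsActionComponent identifies four mesh parts as action components.
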(event OnComponentBeginOverlap(Trigger)
  (params (OverlappedComponent :type Primitive%20Component%20Object%20Reference) (OtherActor :type Actor%20Object%20Reference) (OtherComp :type Primitive%20Component%20Object%20Reference) (OtherBodyIndex :type Integer) (bFromSweep :type Boolean) (SweepResult :type Hit%20Result%20Structure%20%28by%20ref%29))
  (bind _asbp_my_book_key (Utilities|Casting|CastToBP_MyBookKey OtherActor))
  (if (Utilities|Array|ContainsItem (Variables|Default|GetBookKey_0) _asbp_my_book_key)
    (Variables|Default|SetWasHitByKey true)))

(event OnComponentEndOverlap(Trigger)
  (params (OverlappedComponent :type Primitive%20Component%20Object%20Reference) (OtherActor :type Actor%20Object%20Reference) (OtherComp :type Primitive%20Component%20Object%20Reference) (OtherBodyIndex :type Integer))
  (bind _asbp_my_book_key (Utilities|Casting|CastToBP_MyBookKey OtherActor))
  (if (Utilities|Array|ContainsItem (Variables|Default|GetBookKey_0) _asbp_my_book_key)
    (Variables|Default|SetWasHitByKey false)))

(event EventBeginPlay)

(event Collision|EventActorBeginOverlap
  (params (OtherActor :type Actor%20Object%20Reference)))

(event EventTick
  (params (DeltaSeconds :type Float%20%28single-precision%29))
  (if (Variables|Default|GetWasHitByKey)
    (if (Variables|/Hogalaga/MySHIT/My_Bps/BP_MyBookKey.BP_MyBookKey_C|GetHaspickedUp (stale OnComponentBeginOverlap(Trigger) _asbp_my_book_key))
      (if (Utilities|Enum|Equal(Enum) (Variables|/Script/HelloNeighbor.FlatComponent|GetMode (Variables|/Script/HelloNeighbor.FlatActor|GetFlatComponent (stale OnComponentBeginOverlap(Trigger) _asbp_my_book_key))) "FM_Free")
        (Variables|Default|SetMoveDoor true)))
    (else
      (Utilities|FlowControl|Delay 0.5)
      (Variables|Default|SetMoveDoor false))))

(fn ConstructionScript)

(fn OnIsActionComponent
  (params (Component :type Primitive%20Component%20Object%20Reference))
  (return (Math|Boolean|ORBoolean (== Component (Variables|Default|GetPart1StaticMeshComponent)) (== Component (Variables|Default|GetPart2StaticMeshComponent)) (== Component (Variables|Default|GetPart3StaticMeshComponent)) (== Component (Variables|Default|GetPart4StaticMeshComponent)))))