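; BP_NothingToSeeHere is a world text sign with two configurable lines that show or hide when a BP_Human enters or leaves its trigger.
; BeginPlay applies the text, size, color and starting visibility to both text renders.
; Overlap events use flags to choose reveal on first or every entry and hiding on enter or exit.
; Some hide paths set WantDestroyed, which Tick polls to destroy only the trigger component when DetroyActor is set.
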(event OnComponentEndOverlap(Trigger)
  (params (OverlappedComponent :type Primitive%20Component%20Object%20Reference) (OtherActor :type Actor%20Object%20Reference) (OtherComp :type Primitive%20Component%20Object%20Reference) (OtherBodyIndex :type Integer))
  (bind _textrender (Variables|Default|GetTextRender))
  (Utilities|Casting|CastToBP_Human OtherActor)
  (Utilities|FlowControl|Sequence
    (:then_0
      (if (Variables|Default|GetVisibilityOnPlay)
        (if (Variables|Default|GetWantItGoneOnExt)
          (Variables|Default|SetHAsEntered true)
          (Rendering|SetVisibility _textrender false false)
          (Variables|Default|SetWantDestroyed true))
        (else
          (Variables|Default|SetHAsEntered true)
          (Rendering|SetVisibility _textrender false false))))))

(event OnComponentBeginOverlap(Trigger)
  (params (OverlappedComponent :type Primitive%20Component%20Object%20Reference) (OtherActor :type Actor%20Object%20Reference) (OtherComp :type Primitive%20Component%20Object%20Reference) (OtherBodyIndex :type Integer) (bFromSweep :type Boolean) (SweepResult :type Hit%20Result%20Structure%20%28by%20ref%29))
  (bind _textrender (Variables|Default|GetTextRender))
  (Utilities|Casting|CastToBP_Human OtherActor)
  (Utilities|FlowControl|Sequence
    (:then_0
      (if (not (Variables|Default|GetVisibilityOnPlay))
        (if (not (Variables|Default|GetHAsEntered))
          (Rendering|SetVisibility _textrender true false :!label _label))))
    (:then_1
      (if (Variables|Default|GetWantItGoneOnEnter)
        (Rendering|SetVisibility _textrender false false)
        (Variables|Default|SetWantDestroyed true)))
    (:then_2
      (if (not (Variables|Default|GetVisibilityOnPlay))
        (if (Variables|Default|GetEnterOn)
          (goto _label))))))

(event EventBeginPlay
  (bind _textrender (Variables|Default|GetTextRender))
  (Utilities|FlowControl|Sequence
    (:then_0
      (Rendering|SetVisibility _textrender (Variables|Default|GetVisibilityOnPlay) false)
      (Rendering|Components|TextRender|SetText _textrender (Utilities|Text|ToText(String) (Variables|Default|GetText)))
      (Rendering|Components|TextRender|SetText (Variables|Default|GetSecondLine) (Utilities|Text|ToText(String) (Variables|Default|GetSecondLineText)))
      (Rendering|Components|TextRender|SetWorldSize _textrender (Variables|Default|GetSize))
      (Rendering|Components|TextRender|SetTextRenderColor _textrender (Math|Conversions|ToColor(LinearColor) (Variables|Default|GetColor))))))

(event EventTick
  (params (DeltaSeconds :type Float%20%28single-precision%29))
  (if (Variables|Default|GetWantDestroyed)
    (if (Variables|Default|GetDetroyActor)
      (Components|DestroyComponent (Variables|Default|GetTrigger)))))

(fn ConstructionScript)