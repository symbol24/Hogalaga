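; BP_Cupboard2 is an interactive two-door cupboard that swings open and closed when either door part is triggered.
; An action on either part toggles the door state, even reversing mid-swing, and state changes play open or close sound cues.
; Tick advances an Alpha by Speed and lerps both parts between start and end rotations until fully open or closed.
; The construction script poses the doors to match the initial state.
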(event EventBeginPlay
  ;[1 1 1] Comment
)

(event EventOnEventAction
  (params (ActionMaker :type Actor%20Object%20Reference) (SpecialComponent :type Primitive%20Component%20Object%20Reference))
  ;[1 1 1] Comment
  (if (or (== SpecialComponent (Variables|Default|GetRightPart)) (== SpecialComponent (Variables|Default|GetLeftPart)))
    (switch Utilities|FlowControl|Switch|SwitchonEDoorState (Class|Cupboard|GetDoorState)
      (:DS_OPEN
        (Class|Cupboard|SetDoorState "DS_CLOSING" :!label _label))
      (:DS_CLOSING
        (Class|Cupboard|SetDoorState "DS_OPENING" :!label _label_2))
      (:DS_CLOSE
        (goto _label_2))
      (:DS_OPENING
        (goto _label)))))

(event EventTick
  (params (DeltaSeconds :type Float%20%28single-precision%29))
  (bind _speed (Variables|Default|GetSpeed))
  (bind _returnvalue (* DeltaSeconds _speed))
  ;[1 1 1] Comment
  (switch Utilities|FlowControl|Switch|SwitchonEDoorState (Class|Cupboard|GetDoorState)
    (:DS_CLOSING
      (bind _output_get (Variables|Default|SetAlpha (- (Variables|Default|GetAlpha) _returnvalue)))
      (if (<= _output_get 0.0)
        (Variables|Default|SetAlpha 0.0)
        (Class|Cupboard|SetDoorState "DS_CLOSE")))
    (:DS_OPENING
      (bind _output_get_2 (Variables|Default|SetAlpha (+ _returnvalue (Variables|Default|GetAlpha))))
      (if (>= _output_get_2 1.0)
        (Variables|Default|SetAlpha 1.0)
        (Class|Cupboard|SetDoorState "DS_OPEN"))))
  (Transformation|SetRelativeRotation (Variables|Default|GetLeftPart) (Math|Rotator|Lerp(Rotator) (Variables|Default|GetLeftStart) (Variables|Default|GetLeftEnd) (Variables|Default|GetAlpha)) false false)
  (Transformation|SetRelativeRotation (Variables|Default|GetRightPart) (Math|Rotator|Lerp(Rotator) (Variables|Default|GetRightStart) (Variables|Default|GetRightEnd) (Variables|Default|GetAlpha)) false false))

(event EventOnChangeDoorState
  (params (NewState :type EDoorState%20Enum :default "DS_OPEN"))
  ;[1 1 1] Comment
  (switch Utilities|FlowControl|Switch|SwitchonEDoorState NewState
    (:DS_CLOSING
      (Audio|Components|Audio|Play (Variables|Default|Getwood_cupboard_closed_Cue) 0.0))
    (:DS_OPENING
      (Audio|Components|Audio|Play (Variables|Default|Getwood_cupboard_open_Cue) 0.0))))

(fn ConstructionScript
  (switch Utilities|FlowControl|Switch|SwitchonEDoorState (Class|Cupboard|GetDoorState)
    (:DS_OPEN
      (Transformation|SetRelativeRotation (Variables|Default|GetLeftPart) (Variables|Default|GetLeftEnd) false false)
      (Transformation|SetRelativeRotation (Variables|Default|GetRightPart) (Variables|Default|GetRightEnd) false false)
      (Variables|Default|SetAlpha 1.0))
    (:DS_CLOSE
      (Transformation|SetRelativeRotation (Variables|Default|GetLeftPart) (Variables|Default|GetLeftStart) false false)
      (Transformation|SetRelativeRotation (Variables|Default|GetRightPart) (Variables|Default|GetRightStart) false false)
      (Variables|Default|SetAlpha 0.0))))

(fn OnIsActionComponent
  (params (Component :type Primitive%20Component%20Object%20Reference))
  (return (or (== Component (Variables|Default|GetRightPart)) (== Component (Variables|Default|GetLeftPart)))))